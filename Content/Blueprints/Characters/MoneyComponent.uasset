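; Actor component that tracks the owner's money, which exists as an Item_Money stack in the owner's StorageComponent.
; On BeginPlay and on every inventory update it finds that item, reusing the cached one if still in that storage, and caches its count, or zero when none exists.
; SendMoney transfers a given count into another MoneyComponent's storage and reports whether placement succeeded.
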(event `self.ReceiveBeginPlay`
  (bind _output_get (set `self.OwnersStorage` (`Actor.GetComponentByClass` (`self.GetOwner`) "/Game/Blueprints/Storage/StorageComponent.StorageComponent_C")))
  (add `/Game/Blueprints/Storage/StorageComponent.InventoryUpdated` _output_get (delegate `InventoryUpdated`))
  (`self.FindMoney` :!label _label))

(event `InventoryUpdated`
  (goto _label))

(fn `FindMoney`
  (returns (Found :type Boolean) (MoneyItem :type "/Game/Blueprints/Storage/Items/Other/Item_Money Object Reference"))
  (bind _moneyitem (`self.MoneyItem`))
  (bind (_wasfound _item) (`/Game/Blueprints/Storage/StorageComponent.GetItemInStorageByClass` (`self.OwnersStorage`) "/Game/Blueprints/Storage/Items/Other/Item_Money.Item_Money_C"))
  (`/Engine/EditorBlueprintResources/StandardMacros.IsValid` _moneyitem
    (:`Is Valid`
      (if (== (`.Storage` (`/Game/Blueprints/Storage/Items/StorageItem.IsInStorage` _moneyitem)) (`self.OwnersStorage`))
        (set `self.Money` (`/Game/Blueprints/Storage/Items/StorageItem.Count` _moneyitem))
        (return true (`self.MoneyItem`))
        (else
          _)))
    (:`Is Not Valid`
      _))
  (if _wasfound
    (bind _asitem_money (cast `/Game/Blueprints/Storage/Items/Other/Item_Money` _item)
      (:`then`
        (bind _output_get (set `self.MoneyItem` _asitem_money))
        (set `self.Money` (`/Game/Blueprints/Storage/Items/StorageItem.Count` _output_get))
        (return true _output_get))
      (:`CastFailed`
        _)))
  (set `self.Money` 0)
  (set `self.MoneyItem` null)
  (return false null))

(fn `GetMoney`
  (returns (Money :type Integer) (MoneyItem :type "/Game/Blueprints/Storage/Items/Other/Item_Money Object Reference"))
  (return (`self.Money`) (`self.MoneyItem`)))

(fn `SendMoney`
  (params (OtherMoneyComponent :type "/Game/Blueprints/Characters/MoneyComponent Object Reference") (Count :type Integer))
  (returns (Success :type Boolean))
  (if (!= Count 0)
    (bind _placed (`/Game/Blueprints/Storage/StorageComponent.PlaceToAnotherStorage` (`self.OwnersStorage`) (`self.MoneyItem`) (`/Game/Blueprints/Characters/MoneyComponent.OwnersStorage` OtherMoneyComponent) false Count))
    (return _placed)
    (else
      (return true))))