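; Base-style construction actor that can be placed, rotated in yaw steps and broken back into its resources.
; Placement mode disables actor collision and takes its location from the look-at hit.
; Breaking traces down from the bounds center to find the ground, spawns each resource item with its count just above that point, then destroys the actor.
; The break step also draws debug visuals for the bounds and trace.
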(fn `BreakConstruction`
  (locals (L_GroundPoint :type "Vector Structure" :default (0.0 0.0 0.0)))
  (bind (_origin _boxextent) (`self.GetActorBounds` true))
  (`KismetSystemLibrary.DrawDebugBox` _origin _boxextent (struct :`R` 0.06 :`G` 0.06 :`B` 0.06 :`A` 1.0) (struct) 10.0 2.0)
  (bind _outhit (`KismetSystemLibrary.LineTraceSingle` :`Start` (+ _origin (0.0 0.0 0.0)) :`End` (- _origin (0.0 0.0 9999.0)) :`TraceChannel` "TraceTypeQuery1" :`DrawDebugType` "ForDuration"))
  (set `local.L_GroundPoint` (`.Location` (`GameplayStatics.BreakHitResult` _outhit)))
  (`self.SetActorEnableCollision` false)
  (for _array_element (`self.Resources`)
    (bind (_item _count) (break `/Game/Blueprints/Storage/St_ClassItemInfo` _array_element))
    (`|SpawnActorFromClass` _item (`KismetMathLibrary.MakeTransform` (+ (`local.L_GroundPoint`) (0.0 0.0 30.0))) "AlwaysSpawn" "OverrideRootScale" null _count))
  (`self.K2_DestroyActor`))

(fn `GetPlacementLocation`
  (params (LookAtHit :type "HitResult Structure"))
  (returns (Location :type "Vector Structure"))
  (return (`.Location` (`GameplayStatics.BreakHitResult` LookAtHit))))

(fn `RotateConstruction`
  (params (Right :type Boolean))
  (bind _rotatedelta (`self.RotateDelta`))
  (`self.K2_AddActorWorldRotation` (`KismetMathLibrary.MakeRotator` 0.0 0.0 (`KismetMathLibrary.SelectFloat` _rotatedelta (* _rotatedelta -1.0) Right))))

(fn `TogglePlacement`
  (params (Active :type Boolean))
  (set `self.Placing` Active)
  (`self.SetActorEnableCollision` (not (`self.Placing`))))

(fn `UserConstructionScript`)