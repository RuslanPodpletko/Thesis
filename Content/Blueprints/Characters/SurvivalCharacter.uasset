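; Survival character Blueprint that handles damage, death, sprint eligibility and weapon use through HealthStats and EquipComponent.
; Armor scales down incoming damage, and landings deal fixed damage when vertical distance from the saved jump or ledge point is too large, unless climbing.
; HealthEnd triggers death: input is disabled, the mesh ragdolls, CharDead fires and a delayed destroy starts.
; Weapon use supports a melee mode for ranged weapons.
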(event `self.OnWalkingOffLedge`
  (params (PreviousFloorImpactNormal :type "Vector Structure (by ref)") (PreviousFloorContactNormal :type "Vector Structure (by ref)") (PreviousLocation :type "Vector Structure (by ref)") (TimeDelta :type "Float (single-precision)"))
  ;[1 1 1] On jump
  (set `self.Loc` (`self.K2_GetActorLocation`) :!label _label))

(event `self.OnJumped`
  ;[1 1 1] On jump
  (goto _label))

(event `self.ReceiveAnyDamage`
  (params (Damage :type "Float (single-precision)") (DamageType :type "DamageType Object Reference") (InstigatedBy :type "Controller Object Reference") (DamageCauser :type "Actor Object Reference"))
  ;[1 1 1] Damage
  (`/Game/Blueprints/Characters/HealthStats.ChangeHealth` (`self.HealthStats`) (* (/ Damage (/ (+ (`self.ArmorValue`) 20.0) 20.0)) -1.0)))

(event `self.OnLanded`
  (params (Hit :type "HitResult Structure (by ref)"))
  (bind _loc (`self.Loc`))
  ;[1 1 1] Land damage
  (if (not (`self.Climbing`))
    (if (!= (`KismetMathLibrary.VSize` _loc) 0.0)
      (if (> (`KismetMathLibrary.VSize` (* (- _loc (`.Location` (`GameplayStatics.BreakHitResult` Hit))) (0.0 0.0 1.0))) 500.0)
        (`/Game/Blueprints/Characters/HealthStats.ChangeHealth` (`self.HealthStats`) -50.0)))))

(event `self.HealthStats.HealthEnd`
  ;[1 1 1] Damage
  (`self.Death`))

(fn `CanSprint`
  (returns (ReturnValue :type Boolean))
  (return (and (not (`self.Crouching`)) (> (`/Game/Blueprints/Characters/HealthStats.Stamina` (`self.HealthStats`)) 5.0))))

(fn `Death`
  (set `self.Dead` true)
  (`KismetSystemLibrary.PrintString` "DEAD" true true (struct :`R` 1.0 :`G` 0.007289 :`A` 1.0) 3.0)
  (`self.DisableInput` (`GameplayStatics.GetPlayerController` 0))
  (`self.EnableRagdoll`)
  (`self.CharDead` self)
  (`self.SetLifeSpan` (`self.DeathDestroyDelay`)))

(fn `EnableRagdoll`
  (returns (Enabled :type Boolean))
  (`PrimitiveComponent.SetCollisionEnabled` (`self.CapsuleComponent`) "NoCollision")
  (`PrimitiveComponent.SetSimulatePhysics` (`self.Mesh`) true)
  (`PrimitiveComponent.SetCollisionEnabled` (`self.Mesh`) "QueryAndPhysics")
  (`PrimitiveComponent.SetCollisionResponseToAllChannels` (`self.Mesh`) "ECR_Block")
  (`PrimitiveComponent.SetCollisionResponseToChannel` (`self.Mesh`) "ECC_Pawn" "ECR_Ignore")
  (return true))

(fn `GetInteractionInfo`
  (params (Distance :type "Float (double-precision)"))
  (returns (Hit :type "HitResult Structure"))
  (return))

(fn `ShootFromWeapon`
  (params (Shoot :type Boolean) (AsMelee :type Boolean))
  (returns (Shot :type Boolean))
  (bind _weapon (`/Game/Blueprints/Characters/EquipComponent.Weapon` (`self.EquipComponent`)))
  (`/Engine/EditorBlueprintResources/StandardMacros.IsValid` _weapon
    (:`Is Valid`
      (bind _asrange_weapon (cast `/Game/Blueprints/Storage/Items/Equipables/Weapons/RangeWeapon` _weapon)
        (:`then`
          (if AsMelee
            (bind _used (`/Game/Blueprints/Storage/Items/Equipables/Weapons/RangeWeapon.UseAsMeleeWeapon` _asrange_weapon Shoot))
            (return _used)
            (else
              _)))
        (:`CastFailed`
          _))
      (bind _used_2 (`/Game/Blueprints/Storage/Items/Equipables/Weapons/Weapon.UseWeapon` (`/Game/Blueprints/Characters/EquipComponent.Weapon` (`self.EquipComponent`)) Shoot))
      (return _used_2))
    (:`Is Not Valid`
      (return false))))

(fn `UserConstructionScript`
  (set `CharacterMovementComponent.MaxWalkSpeed` (`self.WalkingSpeed`) (`self.CharacterMovement`)))