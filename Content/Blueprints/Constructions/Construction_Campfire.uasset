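; Campfire construction for a survival game that serves as a crafting station and hurts actors standing in it.
; Capsule overlaps maintain a list of affected actors and run a looping timer that applies damage to each, cleared when the list empties.
; Interacting opens the player controller's craft widget, initialized with the campfire's storage and craft components, and fails for characters without a survival player controller.
; The damage tick still prints a debug string.
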(event `self.Capsule.OnComponentBeginOverlap`
  (params (OverlappedComponent :type "PrimitiveComponent Object Reference") (OtherActor :type "Actor Object Reference") (OtherComp :type "PrimitiveComponent Object Reference") (OtherBodyIndex :type Integer) (bFromSweep :type Boolean) (SweepResult :type "HitResult Structure (by ref)"))
  (`KismetArrayLibrary.Array_AddUnique` (`self.ActorsDamaging`) OtherActor)
  (if (not (`KismetSystemLibrary.K2_IsValidTimerHandle` (`self.DamageTimer`)))
    (bind _returnvalue (`KismetSystemLibrary.K2_SetTimer` null "DamageActors" (`self.DamageDelay`) true))
    (set `self.DamageTimer` _returnvalue)))

(event `self.Capsule.OnComponentEndOverlap`
  (params (OverlappedComponent :type "PrimitiveComponent Object Reference") (OtherActor :type "Actor Object Reference") (OtherComp :type "PrimitiveComponent Object Reference") (OtherBodyIndex :type Integer))
  (bind _actorsdamaging (`self.ActorsDamaging`))
  (`KismetArrayLibrary.Array_RemoveItem` _actorsdamaging OtherActor)
  (if (== (`KismetArrayLibrary.Array_Length` _actorsdamaging) 0)
    (`KismetSystemLibrary.K2_ClearAndInvalidateTimerHandle` (`self.DamageTimer`))))

(fn `DamageActors`
  (locals (L_actors :type "Array of Actor Object Reference"))
  (`KismetSystemLibrary.PrintString` "Hello")
  (for _array_element (`self.ActorsDamaging`)
    (`GameplayStatics.ApplyDamage` _array_element (`self.Damage`) null self)))

(fn `Interact`
  (params (Character :type "/Game/Blueprints/Characters/SurvivalCharacter Object Reference"))
  (returns (Successfull :type Boolean) (Message :type String))
  (bind _assurvival_player_controller (cast `/Game/Blueprints/Gamemode/SurvivalPlayerController` (`Pawn.GetController` Character))
    (:`then`
      (bind _craftwidget (`/Game/Blueprints/Gamemode/SurvivalPlayerController.CraftWidget` _assurvival_player_controller true))
      (`/Game/UI/Craft/W_Craft_CraftWindow.InitCraftInterface` _craftwidget (`self.StorageComponent`) (`self.CraftComponent`))
      (return true ""))
    (:`CastFailed`
      (return false "Character is not controlled by player"))))

(fn `ToggleInteractAttempt`
  (params (Enable :type Boolean) (Character :type "/Game/Blueprints/Characters/SurvivalCharacter Object Reference") (Hit :type "HitResult Structure"))
  (returns (ReturnValue :type Boolean))
  (return false))

(fn `UserConstructionScript`)