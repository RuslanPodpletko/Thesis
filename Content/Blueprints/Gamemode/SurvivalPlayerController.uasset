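; Survival player controller that creates the HUD and manages the UI windows: inventory, item exchange, crafting, trading, construction list, dialog and pause menu.
; Each window function creates or removes its widget and calls UIControl, which switches input mode, cursor and pawn input.
; Keys toggle inventory and pause, open the construction list, and Escape or Backspace closes open windows other than inventory and pause menu.
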(event `self.ReceiveBeginPlay`
  (`|ExecutionSequence`
    (:`then_0`
      (bind _returnvalue (`|CreateWidget` "/Game/UI/MainHUD/W_HUD.W_HUD_C" self))
      (bind _output_get (set `self.W_Hud` _returnvalue))
      (`UserWidget.AddToViewport` _output_get 0))
    (:`then_1`
      (`KismetSystemLibrary.Delay` 1.0)
      (`WidgetBlueprintLibrary.SetInputMode_GameOnly` self)
      (set `self.bShowMouseCursor` false))))

(event `Key|C`
  (params (Key :type "Key Structure" :default "AnyKey"))
  (:`Pressed`
    (`/Engine/EditorBlueprintResources/StandardMacros.IsValid` (`self.W_ConstructionList`)
      (:`Is Not Valid`
        (`self.ConstructionList` true)))))

(event `Key|One` :paused true
  (params (Key :type "Key Structure" :default "AnyKey"))
  (:`Pressed`
    (`/Engine/EditorBlueprintResources/StandardMacros.IsValid` (`self.W_PauseMenu`)
      (:`Is Valid`
        (`self.PauseMenu` false))
      (:`Is Not Valid`
        (`self.PauseMenu` true)))))

(event `Key|I`
  (params (Key :type "Key Structure" :default "AnyKey"))
  (:`Pressed`
    (`self.ToggleInventory`)))

(event `Key|BackSpace`
  (params (Key :type "Key Structure" :default "AnyKey"))
  (:`Pressed`
    (`|ExecutionSequence` :!label _label
      (:`then_0`
        (`/Engine/EditorBlueprintResources/StandardMacros.IsValid` (`self.W_ExchangeWidget`)
          (:`Is Valid`
            (`self.ExchangeWidget` null true))))
      (:`then_1`
        (`/Engine/EditorBlueprintResources/StandardMacros.IsValid` (`self.W_CraftWidget`)
          (:`Is Valid`
            (`self.CraftWidget` false))))
      (:`then_2`
        (`/Engine/EditorBlueprintResources/StandardMacros.IsValid` (`self.W_TradeWidget`)
          (:`Is Valid`
            (`self.TraderWidget` null true))))
      (:`then_3`
        (`/Engine/EditorBlueprintResources/StandardMacros.IsValid` (`self.W_ConstructionList`)
          (:`Is Valid`
            (`self.ConstructionList` false))))
      (:`then_4`
        (`/Engine/EditorBlueprintResources/StandardMacros.IsValid` (`self.W_Dialog`)
          (:`Is Valid`
            (`self.DialogWidget` false)))))))

(event `Key|Escape`
  (params (Key :type "Key Structure" :default "AnyKey"))
  (:`Pressed`
    (goto _label)))

(fn `ConstructionList`
  (params (Show :type Boolean))
  (if Show
    (bind _returnvalue (`|CreateWidget` "/Game/UI/Constructions/W_ConstructionList.W_ConstructionList_C" self))
    (bind _output_get (set `self.W_ConstructionList` _returnvalue))
    (`UserWidget.AddToViewport` _output_get 0)
    (`self.UIControl` true (`self.W_TradeWidget`))
    (else
      (`Widget.RemoveFromParent` (`self.W_ConstructionList`))
      (`self.WindowClosed` (`self.W_ConstructionList`))
      (set `self.W_ConstructionList` null)
      (`self.UIControl` false))))

(fn `CraftWidget`
  (params (Show :type Boolean))
  (returns (CraftWidget :type "/Game/UI/Craft/W_Craft_CraftWindow Object Reference"))
  (if Show
    (bind _returnvalue (`|CreateWidget` "/Game/UI/Craft/W_Craft_CraftWindow.W_Craft_CraftWindow_C" self))
    (bind _output_get (set `self.W_CraftWidget` _returnvalue))
    (`UserWidget.AddToViewport` _output_get 0)
    (`self.UIControl` true (`self.W_CraftWidget`))
    (set `self.W_CurrentWidget` (`self.W_CraftWidget`))
    (return (`self.W_CraftWidget`))
    (else
      (`Widget.RemoveFromParent` (`self.W_CraftWidget`))
      (`self.WindowClosed` (`self.W_CraftWidget`))
      (set `self.W_CraftWidget` null)
      (set `self.W_CurrentWidget` null)
      (`self.UIControl` false)
      (return null))))

(fn `DialogWidget`
  (params (Show :type Boolean) (DialogTree :type "/Game/Blueprints/Characters/Dialog/DialogTrees/DialogTree Object Reference") (DialogComponent :type "/Game/Blueprints/Characters/Dialog/DialogComponent Object Reference"))
  (if Show
    (bind _returnvalue (`|CreateWidget` "/Game/UI/Dialog/W_Dialog.W_Dialog_C" self DialogTree DialogComponent))
    (bind _output_get (set `self.W_Dialog` _returnvalue))
    (`UserWidget.AddToViewport` _output_get 0)
    (`self.UIControl` true (`self.W_Dialog`))
    (set `self.W_CurrentWidget` (`self.W_Dialog`))
    (else
      (`Widget.RemoveFromParent` (`self.W_Dialog`))
      (`self.WindowClosed` (`self.W_Dialog`))
      (set `self.W_Dialog` null)
      (set `self.W_CurrentWidget` null)
      (`self.UIControl` false))))

(fn `ExchangeWidget`
  (params (ExchangeComponent :type "/Game/Blueprints/Storage/StorageComponent Object Reference") (Remove :type Boolean))
  (if Remove
    (bind _w_exchangewidget (`self.W_ExchangeWidget`)
      (:`then`
        (`Widget.RemoveFromParent` _w_exchangewidget)
        (`self.WindowClosed` (`self.W_ExchangeWidget`))
        (set `self.W_ExchangeWidget` null)
        (set `self.W_CurrentWidget` null)
        (`self.UIControl` false))
      (:`else`))
    (else
      (bind _returnvalue (`|CreateWidget` "/Game/UI/Inventory/W_ItemExchange.W_ItemExchange_C" self ExchangeComponent))
      (bind _output_get (set `self.W_ExchangeWidget` _returnvalue))
      (`UserWidget.AddToViewport` _output_get 0)
      (`self.UIControl` true (`self.W_ExchangeWidget`))
      (set `self.W_CurrentWidget` (`self.W_ExchangeWidget`)))))

(fn `PauseMenu`
  (params (Show :type Boolean))
  (if Show
    (bind _returnvalue (`|CreateWidget` "/Game/UI/MainMenu/W_PauseMenu.W_PauseMenu_C" self))
    (bind _output_get (set `self.W_PauseMenu` _returnvalue))
    (`UserWidget.AddToViewport` _output_get 0)
    (`self.UIControl` true (`self.W_PauseMenu`))
    (`GameplayStatics.SetGamePaused` true)
    (else
      (`/Engine/EditorBlueprintResources/StandardMacros.IsValid` (`self.W_PauseMenu`)
        (:`Is Valid`
          (`Widget.RemoveFromParent` (`self.W_PauseMenu`))
          (set `self.W_PauseMenu` null)
          (`self.UIControl` false)
          (`GameplayStatics.SetGamePaused` false))))))

(fn `ToggleInventory`
  (if (not (`self.InventoryShown`))
    ;[1 1 1] Show inventory, block character input
    (bind _returnvalue (`|CreateWidget` "/Game/UI/Inventory/W_Inventory.W_Inventory_C" self))
    (bind _output_get (set `self.W_Inventory` _returnvalue))
    (`UserWidget.AddToViewport` _output_get 0)
    (`/Game/UI/Inventory/W_Inventory.InventoryAddedToViewport` (`self.W_Inventory`))
    (set `self.InventoryShown` true)
    (`self.UIControl` true (`self.W_Inventory`))
    (set `self.W_CurrentWidget` (`self.W_Inventory`))
    (else
      ;[1 1 1] Hide widget, return inputs
      (`Widget.RemoveFromParent` (`self.W_Inventory`))
      (set `self.InventoryShown` false)
      (`self.UIControl` false)
      (set `self.W_CurrentWidget` null)
      (`self.WindowClosed` (`self.W_Inventory`))
      (set `self.W_Inventory` null))))

(fn `TraderWidget`
  (params (TradeComponent :type "/Game/Blueprints/Characters/Trade/TradeComponent Object Reference") (Remove :type Boolean))
  (if Remove
    (`Widget.RemoveFromParent` (`self.W_TradeWidget`))
    (`self.WindowClosed` (`self.W_TradeWidget`))
    (set `self.W_TradeWidget` null)
    (`self.UIControl` false)
    (set `self.W_CurrentWidget` null)
    (else
      (bind _returnvalue (`|CreateWidget` "/Game/UI/Inventory/W_ItemTrade.W_ItemTrade_C" self TradeComponent))
      (bind _output_get (set `self.W_TradeWidget` _returnvalue))
      (`UserWidget.AddToViewport` _output_get 0)
      (`self.UIControl` true (`self.W_TradeWidget`))
      (set `self.W_CurrentWidget` (`self.W_TradeWidget`)))))

(fn `UIControl`
  (params (Activate :type Boolean) (InWidgetToFocus :type "Widget Object Reference"))
  (if Activate
    (set `self.bShowMouseCursor` true)
    (`WidgetBlueprintLibrary.SetInputMode_GameAndUIEx` self InWidgetToFocus "DoNotLock" false)
    (`self.DisableInput` (`self.K2_GetPawn`) self)
    (else
      (set `self.bShowMouseCursor` false)
      (`self.EnableInput` (`self.K2_GetPawn`) self)
      (`WidgetBlueprintLibrary.SetInputMode_GameOnly` self))))

(fn `UserConstructionScript`)