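; Equipment component for survival characters that equips and unequips items in head, torso, legs, feet and weapon slots.
; Clothes follow the character mesh through master pose, while hats and weapons snap to sockets, with events called on changes.
; For players, torso and weapon attach to the first-person or body mesh by active camera.
; View switching reattaches them and hides head, legs and feet in first person.
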(event `self.ReceiveBeginPlay`
  (bind _assurvival_character (cast `/Game/Blueprints/Characters/SurvivalCharacter` (`self.GetOwner`)))
  (bind _output_get (set `self.SurvivalCharacter` _assurvival_character))
  (bind _assurvival_character_player (cast `/Game/Blueprints/Characters/SurvivalCharacter_Player` _output_get))
  (add `/Game/Blueprints/Characters/SurvivalCharacter_Player.ViewSwitched` _assurvival_character_player (`|CreateDelegate` :!event `SwitchMeshesOnView`)))

(event `HideItems`
  (`KismetSystemLibrary.Delay` 0.2))

(fn `AttachClothes`
  (params (Clothes :type "/Game/Blueprints/Storage/Items/Equipables/Clothes/ClothesItem Object Reference"))
  (locals (L_MeshToAttach :type "SkeletalMeshComponent Object Reference"))
  (`/Engine/EditorBlueprintResources/StandardMacros.IsValid` Clothes
    (:`Is Valid`
      (bind _output_get (set `local.L_MeshToAttach` (`self.MeshToAttach` Clothes)))
      (`Actor.K2_AttachToComponent` Clothes _output_get "None" "SnapToTarget" "SnapToTarget" "SnapToTarget" true)
      (`SkinnedMeshComponent.SetLeaderPoseComponent` (`/Game/Blueprints/Storage/Items/Equipables/Clothes/ClothesItem.Clothes` Clothes) (`local.L_MeshToAttach`)))))

(fn `AttachHat`
  (params (Hat :type "/Game/Blueprints/Storage/Items/Equipables/Hats/Hat Object Reference"))
  (`Actor.K2_AttachToComponent` Hat (`self.MeshToAttach` Hat) "Skt_Hat" "SnapToTarget" "SnapToTarget" "SnapToTarget" true))

(fn `AttachWeapon`
  (params (Attach :type Boolean))
  (bind _weapon (`self.Weapon`))
  (`/Engine/EditorBlueprintResources/StandardMacros.IsValid` (`self.Weapon`)
    (:`Is Valid`
      (if Attach
        (`Actor.K2_AttachToComponent` _weapon (`self.MeshToAttach` _weapon) "Skt_Weapon" "SnapToTarget" "SnapToTarget" "SnapToTarget" true)
        (else
          (`Actor.DetachRootComponentFromParent` (`self.Weapon`) true))))))

(fn `EqiupWeapon`
  (params (Item :type "/Game/Blueprints/Storage/Items/Equipables/EquipableItem Object Reference"))
  (bind _asweapon (cast `/Game/Blueprints/Storage/Items/Equipables/Weapons/Weapon` Item))
  (set `self.Weapon` _asweapon)
  (`self.AttachWeapon` true)
  (`self.WeaponEquipped` (`self.Weapon`)))

(fn `EquipClothes`
  (params (Item :type "/Game/Blueprints/Storage/Items/StorageItem Object Reference"))
  (bind _asclothes_item (cast `/Game/Blueprints/Storage/Items/Equipables/Clothes/ClothesItem` Item))
  (`|ExecutionSequence`
    (:`then_0`
      (switch `/Game/Blueprints/Storage/Items/Equipables/E_EquipPart` (`/Game/Blueprints/Storage/Items/Equipables/EquipableItem.EquipPart` _asclothes_item)
        (:`NewEnumerator1`
          (set `self.Torso` _asclothes_item))
        (:`NewEnumerator2`
          (set `self.Legs` _asclothes_item))
        (:`NewEnumerator3`
          (set `self.Foots` _asclothes_item))))
    (:`then_1`
      (`self.AttachClothes` _asclothes_item))))

(fn `EquipHat`
  (params (Item :type "/Game/Blueprints/Storage/Items/StorageItem Object Reference"))
  (bind _ashat (cast `/Game/Blueprints/Storage/Items/Equipables/Hats/Hat` Item))
  (bind _output_get (set `self.Head` _ashat))
  (`self.AttachHat` _output_get))

(fn `EquipItem`
  (params (Item :type "/Game/Blueprints/Storage/Items/Equipables/EquipableItem Object Reference") (Part :type "/Game/Blueprints/Storage/Items/Equipables/E_EquipPart Enum"))
  (returns (Equipped :type Boolean))
  (locals (L_Item :type "/Game/Blueprints/Storage/Items/Equipables/EquipableItem Object Reference"))
  (set `local.L_Item` Item)
  (`self.UnEquipItem` Part)
  (switch `/Game/Blueprints/Storage/Items/Equipables/E_EquipPart` Part
    (:`NewEnumerator0`
      (`self.EquipHat` (`local.L_Item`)))
    (:`NewEnumerator1`
      (`self.EquipClothes` (`local.L_Item`) :!label _label))
    (:`NewEnumerator2`
      (goto _label))
    (:`NewEnumerator3`
      (goto _label))
    (:`NewEnumerator4`
      (`self.EqiupWeapon` (`local.L_Item`))))
  (`|ExecutionSequence`
    (:`then_0`
      ;[1 1 1] Show or hide items at equip
      (switch `/Game/Blueprints/Storage/Items/Equipables/E_EquipPart` (`/Game/Blueprints/Storage/Items/Equipables/EquipableItem.EquipPart` (`local.L_Item`))
        (:`NewEnumerator0`
          (`/Engine/EditorBlueprintResources/StandardMacros.IsValid` (`self.Head`)
            (:`Is Valid`
              (`Actor.SetActorHiddenInGame` (`self.Head`) false)
              (bind _assurvival_character_player (cast `/Game/Blueprints/Characters/SurvivalCharacter_Player` (`self.SurvivalCharacter`) :!label _label_2))
              (`self.SwitchMeshesOnView` (`/Game/Blueprints/Characters/SurvivalCharacter_Player.FirstCameraActive` _assurvival_character_player)))))
        (:`NewEnumerator1`
          (`/Engine/EditorBlueprintResources/StandardMacros.IsValid` (`self.Torso`)
            (:`Is Valid`
              (`Actor.SetActorHiddenInGame` (`self.Torso`) false))))
        (:`NewEnumerator2`
          (`/Engine/EditorBlueprintResources/StandardMacros.IsValid` (`self.Legs`)
            (:`Is Valid`
              (`Actor.SetActorHiddenInGame` (`self.Legs`) false)
              (goto _label_2))))
        (:`NewEnumerator3`
          (`/Engine/EditorBlueprintResources/StandardMacros.IsValid` (`self.Foots`)
            (:`Is Valid`
              (`Actor.SetActorHiddenInGame` (`self.Foots`) false)
              (goto _label_2))))
        (:`NewEnumerator4`
          (`/Engine/EditorBlueprintResources/StandardMacros.IsValid` (`self.Weapon`)
            (:`Is Valid`
              (`Actor.SetActorHiddenInGame` (`self.Weapon`) false))))))
    (:`then_1`
      (`self.ItemEquipped` (`local.L_Item`))
      (return true))))

(fn `MeshToAttach`
  (params (Item :type "/Game/Blueprints/Storage/Items/Equipables/EquipableItem Object Reference"))
  (returns (SkeletalMesh :type "SkeletalMeshComponent Object Reference"))
  (bind _mesh (`Character.Mesh` (`self.SurvivalCharacter`)))
  (bind _assurvival_character_player (cast `/Game/Blueprints/Characters/SurvivalCharacter_Player` (`self.SurvivalCharacter`))
    (:`then`
      (bind _returnvalue (select `bool` (`/Game/Blueprints/Characters/SurvivalCharacter_Player.FirstCameraActive` _assurvival_character_player) :`false` (`Character.Mesh` _assurvival_character_player) :`true` (`/Game/Blueprints/Characters/SurvivalCharacter_Player.FirstPerson` _assurvival_character_player)))
      (return (select `/Game/Blueprints/Storage/Items/Equipables/E_EquipPart` (`/Game/Blueprints/Storage/Items/Equipables/EquipableItem.EquipPart` Item) :`NewEnumerator0` _mesh :`NewEnumerator1` _returnvalue :`NewEnumerator2` _mesh :`NewEnumerator3` _mesh :`NewEnumerator4` _returnvalue)))
    (:`CastFailed`
      (return (`Character.Mesh` (`self.SurvivalCharacter`))))))

(fn `PartEqupped`
  (params (Part :type "/Game/Blueprints/Storage/Items/Equipables/E_EquipPart Enum"))
  (returns (Equipped :type Boolean) (Item :type "/Game/Blueprints/Storage/Items/Equipables/EquipableItem Object Reference"))
  (bind _returnvalue (select `/Game/Blueprints/Storage/Items/Equipables/E_EquipPart` Part :`NewEnumerator0` (`self.Head`) :`NewEnumerator1` (`self.Torso`) :`NewEnumerator2` (`self.Legs`) :`NewEnumerator3` (`self.Foots`) :`NewEnumerator4` (`self.Weapon`) :!type "/Game/Blueprints/Storage/Items/Equipables/EquipableItem Object Reference"))
  (return (`KismetSystemLibrary.IsValid` _returnvalue) _returnvalue))

(fn `SwitchMeshesOnView`
  (params (FirstPirson :type Boolean))
  (locals (L_FirstP :type Boolean) (L_PartItem :type "Actor Object Reference"))
  (set `local.L_FirstP` FirstPirson)
  (`|ExecutionSequence`
    (:`then_0`
      (`self.AttachClothes` (`self.Torso`))
      (`self.AttachWeapon` true))
    (:`then_1`
      (for _index (range 3)
        (bind _output_get (set `local.L_PartItem` (select `int` _index :`0` (`self.Head`) :`1` (`self.Legs`) :`2` (`self.Foots`) :!type "Actor Object Reference")))
        (`/Engine/EditorBlueprintResources/StandardMacros.IsValid` _output_get
          (:`Is Valid`
            (`Actor.SetActorHiddenInGame` (`local.L_PartItem`) (`local.L_FirstP`))))))))

(fn `UnEquipItem`
  (params (Part :type "/Game/Blueprints/Storage/Items/Equipables/E_EquipPart Enum"))
  (returns (Uequipped :type Boolean))
  (locals (L_UnequipItem :type "/Game/Blueprints/Storage/Items/Equipables/EquipableItem Object Reference"))
  (bind (_equipped _item) (`self.PartEqupped` Part))
  (if _equipped
    (set `local.L_UnequipItem` _item)
    (switch `/Game/Blueprints/Storage/Items/Equipables/E_EquipPart` Part
      (:`NewEnumerator0`
        (set `self.Head` null))
      (:`NewEnumerator1`
        (set `self.Torso` null))
      (:`NewEnumerator2`
        (set `self.Legs` null))
      (:`NewEnumerator3`
        (set `self.Foots` null))
      (:`NewEnumerator4`
        (set `self.Weapon` null)))
    (`|ExecutionSequence`
      (:`then_0`
        (bind _asclothes_item (cast `/Game/Blueprints/Storage/Items/Equipables/Clothes/ClothesItem` (`local.L_UnequipItem`)))
        (`SkinnedMeshComponent.SetLeaderPoseComponent` (`/Game/Blueprints/Storage/Items/Equipables/Clothes/ClothesItem.Clothes` _asclothes_item) null))
      (:`then_1`
        (`self.ItemUnEquipped` (`local.L_UnequipItem`))
        (return true)))
    (else
      (return false))))