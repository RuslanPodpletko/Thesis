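; Choppable tree actor that only takes damage from an axe and yields wood once felled.
; Axe hits lower Condition until it marks itself fallen and fires TreeFalls, whose bound handler plays a timeline that pitches the actor over.
; Interacting with the fallen tree adds wood items to the character's storage and destroys the actor.
; The construction script randomizes wood count and mesh scale; berry-drop logic is present but unconnected.
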(event `self.ReceiveBeginPlay`
  (add `self.TreeFalls` (delegate `PlayFallAnim`)))

(event `PlayFallAnim` :!signature `self.TreeFalls`
  (params (Tree :type "/Game/Blueprints/Prefabs/Tree Object Reference") (Instigator :type "Pawn Object Reference"))
  (bind (_returnvalue_roll _returnvalue_pitch _returnvalue_yaw) (`KismetMathLibrary.BreakRotator` (`self.K2_GetActorRotation`)))
  ;[1 1 1] Animation
  (bind (_direction _newtrack_0) (`Timeline|Timeline_0` :!via `PlayFromStart`)
    (:`Update`
      (`self.K2_SetActorRotation` (`KismetMathLibrary.MakeRotator` _returnvalue_roll (`KismetMathLibrary.Lerp` _returnvalue_pitch 90.0 _newtrack_0) _returnvalue_yaw)))))

(event `self.ReceiveAnyDamage`
  (params (Damage :type "Float (single-precision)") (DamageType :type "DamageType Object Reference") (InstigatedBy :type "Controller Object Reference") (DamageCauser :type "Actor Object Reference"))
  ;[1 1 1] Tree hit
  (`self.HitATree` Damage InstigatedBy DamageCauser))

(fn `HitATree`
  (params (Damage :type "Float (double-precision)") (Instigator :type "Controller Object Reference") (Causer :type "Object Object Reference"))
  (returns (Damaged :type Boolean) (Falls :type Boolean))
  (if (== (`GameplayStatics.GetObjectClass` Causer) "/Game/Blueprints/Storage/Items/Equipables/Weapons/Weapon_Axe.Weapon_Axe_C")
    (bind _output_get (set `self.Condition` (- (`self.Condition`) Damage)))
    (if (<= _output_get 0.0)
      (set `self.Fallen` true)
      (`self.TreeFalls` self (`Controller.K2_GetPawn` Instigator))
      (return true true)
      (else
        (return true false)))
    (else
      (return false false))))

(fn `Interact`
  (params (Character :type "/Game/Blueprints/Characters/SurvivalCharacter Object Reference"))
  (returns (Successfull :type Boolean) (Message :type String))
  (if (`self.Fallen`)
    (`/Game/Blueprints/Storage/StorageComponent.CreateItems` (`/Game/Blueprints/Characters/SurvivalCharacter.StorageComponent` Character) (`|MakeArray` (make `/Game/Blueprints/Storage/St_ClassItemInfo` "/Game/Blueprints/Storage/Items/Item_Wood.Item_Wood_C" (`self.WoodCount`))))
    (`self.K2_DestroyActor`)
    (return true "")
    (else
      (return false "Tree is not fallen"))))

(fn `ToggleInteractAttempt`
  (params (Enable :type Boolean) (Character :type "/Game/Blueprints/Characters/SurvivalCharacter Object Reference") (Hit :type "HitResult Structure"))
  (returns (ReturnValue :type Boolean))
  (return false))

(fn `UserConstructionScript`
  (set `self.WoodCount` (`KismetMathLibrary.RandomIntegerInRange` 5 10))
  (`SceneComponent.SetRelativeScale3D` (`self.ScotsPineTall_01`) (* (1.0 1.0 1.0) (`KismetMathLibrary.RandomFloatInRange` 0.7 0.9))))