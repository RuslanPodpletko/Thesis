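; Foundation building piece that chooses where it is placed from the look-at hit, snapping to other foundations.
; GetPlacementLocation searches all foundation actors for a nearby one within a distance band of the hit point, excluding itself.
; When one is found, it offsets one tile from it along the look direction rounded to 90-degree steps; otherwise it returns the hit location.
; A grid-rounding snap helper is left unused.
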(fn `GetPlacementLocation`
  (params (LookAtHit :type "HitResult Structure"))
  (returns (Location :type "Vector Structure"))
  (locals (L_Distance :type "Float (double-precision)" :default 100000000.0) (L_ClosestFundament :type "/Game/Blueprints/Constructions/Constuction_Fundament Object Reference"))
  (bind (_bblockinghit _binitialoverlap _time _location) (`GameplayStatics.BreakHitResult` LookAtHit))
  (bind _outactors (`GameplayStatics.GetAllActorsOfClass` "Constuction_Fundament_C"))
  (for _array_element _outactors
    (if (!= self _array_element)
      (bind _returnvalue (`KismetMathLibrary.VSize` (- (`self.K2_GetActorLocation` _array_element) (`.Location` (`GameplayStatics.BreakHitResult` LookAtHit)))))
      (if (`KismetMathLibrary.InRange_FloatFloat` _returnvalue 50.0 150.0)
        (if (<= _returnvalue (`local.L_Distance`))
          (set `local.L_Distance` _returnvalue)
          (set `local.L_ClosestFundament` _array_element)))))
  (`/Engine/EditorBlueprintResources/StandardMacros.IsValid` (`local.L_ClosestFundament`)
    (:`Is Valid`
      (return (+ (`self.K2_GetActorLocation` (`local.L_ClosestFundament`)) (`KismetMathLibrary.RotateAngleAxis` (100.0 0.0 0.0) (* (`KismetMathLibrary.Round` (/ (.yaw (`KismetMathLibrary.FindLookAtRotation` (`self.K2_GetActorLocation` (`local.L_ClosestFundament`)) _location)) 90.0)) 90.0) (0.0 0.0 1.0)))))
    (:`Is Not Valid`
      (return _location))))

(fn `UserConstructionScript`
  (`parent.UserConstructionScript`))