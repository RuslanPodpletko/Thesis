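; Rock is a harvestable world prefab that yields rock items when mined with a pickaxe.
; Point damage calls RockHit, which ignores any damage causer whose class is not exactly Weapon_Pickaxe.
; Each valid hit decrements the Rocks count and spawns an Item_Rock at the hit location, destroying the actor once the count runs out.
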(event `self.ReceivePointDamage`
  (params (Damage :type "Float (single-precision)") (DamageType :type "DamageType Object Reference") (HitLocation :type "Vector Structure") (HitNormal :type "Vector Structure") (HitComponent :type "PrimitiveComponent Object Reference") (BoneName :type Name) (ShotFromDirection :type "Vector Structure") (InstigatedBy :type "Controller Object Reference") (DamageCauser :type "Actor Object Reference") (HitInfo :type "HitResult Structure (by ref)"))
  (`self.RockHit` DamageCauser HitLocation))

(fn `RockHit`
  (params (DamageCauser :type "Object Object Reference") (HitLocation :type "Vector Structure"))
  (if (== (`GameplayStatics.GetObjectClass` DamageCauser) "/Game/Blueprints/Storage/Items/Equipables/Weapons/Weapon_Pickaxe.Weapon_Pickaxe_C")
    (set `self.Rocks` (- (`self.Rocks`) 1))
    (`|SpawnActorFromClass` "/Game/Blueprints/Storage/Items/Item_Rock.Item_Rock_C" (`KismetMathLibrary.MakeTransform` HitLocation) "AdjustIfPossibleButAlwaysSpawn" "OverrideRootScale" null 1)
    (if (<= (`self.Rocks`) 0)
      (`self.K2_DestroyActor`))))

(fn `UserConstructionScript`)