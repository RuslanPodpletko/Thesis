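; Roof building piece that overrides placement location to snap onto walls or neighboring roofs.
; Aiming at a wall puts the roof above it, offset sideways along the wall's right vector based on the hit's side.
; Otherwise it searches all other roofs for one near the hit and steps one tile from it, with yaw rounded to 90-degree increments.
; With no roof in range, it returns the raw hit location.
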(fn `GetPlacementLocation`
  (params (LookAtHit :type "HitResult Structure"))
  (returns (Location :type "Vector Structure"))
  (locals (L_Distance :type "Float (double-precision)" :default 999999.0) (L_ClosestRoof :type "/Game/Blueprints/Constructions/Constuction_Roof Object Reference") (L_Hit :type "HitResult Structure"))
  (bind (_bblockinghit _binitialoverlap _time _location) (`GameplayStatics.BreakHitResult` (`local.L_Hit`)))
  (set `local.L_Hit` LookAtHit)
  (bind _asconstuction_wall (cast `/Game/Blueprints/Constructions/Constuction_Wall` (`.HitActor` (`GameplayStatics.BreakHitResult` (`local.L_Hit`))))
    (:`then`
      (return (+ (* (`self.GetActorRightVector` _asconstuction_wall) (`KismetMathLibrary.SelectFloat` 40.01 -40.01 (< (`KismetMathLibrary.Dot_VectorVector` (`KismetMathLibrary.GetDirectionUnitVector` (`.Location` (`GameplayStatics.BreakHitResult` (`local.L_Hit`))) (`self.K2_GetActorLocation` _asconstuction_wall)) (`self.GetActorRightVector` _asconstuction_wall)) 0.0))) (`self.K2_GetActorLocation` _asconstuction_wall) (0.0 0.0 280.0))))
    (:`CastFailed`
      (bind _outactors (`GameplayStatics.GetAllActorsOfClass` "Constuction_Roof_C"))
      (for _array_element _outactors
        (if (!= self _array_element)
          (bind _returnvalue (`KismetMathLibrary.VSize` (- (`self.K2_GetActorLocation` _array_element) (`.Location` (`GameplayStatics.BreakHitResult` (`local.L_Hit`))))))
          (if (<= _returnvalue 150.0)
            (if (<= _returnvalue (`local.L_Distance`))
              (set `local.L_Distance` _returnvalue)
              (set `local.L_ClosestRoof` _array_element)))))
      (`/Engine/EditorBlueprintResources/StandardMacros.IsValid` (`local.L_ClosestRoof`)
        (:`Is Valid`
          (return (+ (`self.K2_GetActorLocation` (`local.L_ClosestRoof`)) (`KismetMathLibrary.RotateAngleAxis` (100.0 0.0 0.0) (* (`KismetMathLibrary.Round` (/ (.yaw (`KismetMathLibrary.FindLookAtRotation` (`self.K2_GetActorLocation` (`local.L_ClosestRoof`)) _location)) 90.0)) 90.0) (0.0 0.0 1.0)))))
        (:`Is Not Valid`
          (return _location))))))

(fn `UserConstructionScript`
  (`parent.UserConstructionScript`))