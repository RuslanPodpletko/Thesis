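; Interactable storage chest construction that opens its lid and shows its storage to the interacting player.
; Interact caches the SurvivalPlayerController and plays a timeline that pitches the Top component open.
; On finish, an Opened toggle gates the exchange widget for StorageComponent and a binding to the controller's window-closed event.
; Closing the window unbinds, clears the controller and reverses the lid animation.
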(event `OpenBox`
  (bind (_direction _lerp) (`Timeline|TopAnimation` :!via `PlayFromStart` :!label _label)
    (:`Update`
      (`SceneComponent.K2_SetRelativeRotation` (`self.Top`) (`KismetMathLibrary.MakeRotator` 0.0 _lerp) false false))
    (:`Finished`
      (bind _output_get (set `self.Opened` (not (`self.Opened`))))
      (if _output_get
        (`/Game/Blueprints/Gamemode/SurvivalPlayerController.ExchangeWidget` (`self.InteractPlayerController`) (`self.StorageComponent`) false)
        (add `/Game/Blueprints/Gamemode/SurvivalPlayerController.WindowClosed` (`self.InteractPlayerController`) (`|CreateDelegate` :!event `WindowClosed_Event`))))))

(event `WindowClosed_Event`
  (params (Widget :type "UserWidget Object Reference"))
  (remove `/Game/Blueprints/Gamemode/SurvivalPlayerController.WindowClosed` (`self.InteractPlayerController`) (delegate `WindowClosed_Event`))
  (set `self.InteractPlayerController` null)
  (goto _label :!via `ReverseFromEnd`))

(fn `Interact`
  (params (Character :type "/Game/Blueprints/Characters/SurvivalCharacter Object Reference"))
  (returns (Successfull :type Boolean) (Message :type String))
  (bind _assurvival_player_controller (cast `/Game/Blueprints/Gamemode/SurvivalPlayerController` (`Pawn.GetController` Character))
    (:`then`
      (set `self.InteractPlayerController` _assurvival_player_controller)
      (`self.OpenBox`)
      (return true ""))
    (:`CastFailed`
      (return false ""))))

(fn `ToggleInteractAttempt`
  (params (Enable :type Boolean) (Character :type "/Game/Blueprints/Characters/SurvivalCharacter Object Reference") (Hit :type "HitResult Structure"))
  (returns (ReturnValue :type Boolean))
  (return false))

(fn `UserConstructionScript`)