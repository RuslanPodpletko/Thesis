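; Survival game mode that notifies the game instance when a level opens and exposes the world's time of day.
; On BeginPlay it calls OpenedLevel on the SurvivalGameInstance, then caches the first DayNightCircle actor found in the level.
; GetTime returns that actor's Time value, or -1 when no valid day-night actor is cached.
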(event `self.ReceiveBeginPlay`
  (`|ExecutionSequence`
    (:`then_0`
      (bind _assurvival_game_instance (cast `/Game/Blueprints/Gamemode/SurvivalGameInstance` (`GameplayStatics.GetGameInstance`)))
      (`/Game/Blueprints/Gamemode/SurvivalGameInstance.OpenedLevel` _assurvival_game_instance))
    (:`then_1`
      (bind _outactors (`GameplayStatics.GetAllActorsOfClass` "/Game/Blueprints/Other/DayNightCircle/DayNightCircle.DayNightCircle_C"))
      (set `self.DayHightCircle` (`KismetArrayLibrary.Array_Get` _outactors)))))

(fn `GetTime`
  (returns (Time :type "Float (double-precision)"))
  (bind _dayhightcircle (`self.DayHightCircle`)
    (:`then`
      (return (`/Game/Blueprints/Other/DayNightCircle/DayNightCircle.Time` _dayhightcircle)))
    (:`else`
      (return -1.0))))

(fn `UserConstructionScript`)