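; RPGStats is a Blueprint that tracks a character's experience and level for RPG progression.
; ChangeExperience updates experience and runs a threshold check, which adds one level, calls NextLevel and recalculates the next requirement through a rounding math expression.
; The check is a single branch, so each change grants at most one level, and experience is not reset.
; Tick prints level, experience and next threshold on screen every frame.
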(event EventBeginPlay)

(event EventTick
  (params (DeltaSeconds :type Float%20%28single-precision%29))
  (CallFunction|PrintRPGStats))

(fn ChangeExperience
  (params (Experience :type Float%20%28single-precision%29))
  (Variables|Default|SetExperience (+ Experience (Variables|Default|GetExperience)))
  (CallFunction|CheckExpforLevel))

(fn ChangeLevel
  (params (AddLevel :type Integer))
  (Variables|Default|SetLevel (+ AddLevel (Variables|Default|GetLevel))))

(fn CheckExpforLevel
  (if (>= (Variables|Default|GetExperience) (Variables|Default|GetExpForNextLevel))
    (CallFunction|ChangeLevel 1)
    (Default|CallNextLevel)
    (Variables|Default|SetExpForNextLevel (CallFunction|CalculateExpforCurrentLvl))))

(fn CalculateExpforCurrentLvl
  (return (Math|Conversions|ToFloat(Integer) (|((round({ECE0EAF4-49EF-776E-3CE2-D482D42B2659}))+({BBF5A053-4D85-C077-DFD5-8F9D95499C0A}*100))))))

(fn PrintRPGStats
  (Utilities|FlowControl|Sequence
    (:then_0
      (Development|PrintString (Utilities|String|Append "Exp to next Lvl: " (Utilities|String|ToString(Float) (Variables|Default|GetExpForNextLevel))) true true "(R=1.000000,G=1.000000,B=1.000000,A=1.000000)" 0.0))
    (:then_1
      (Development|PrintString (Utilities|String|Append "Exp: " (Utilities|String|ToString(Float) (Variables|Default|GetExperience))) true true "(R=1.000000,G=1.000000,B=1.000000,A=1.000000)" 0.0))
    (:then_2
      (Development|PrintString (Utilities|String|Append "Level: " (Utilities|String|ToString(Integer) (Variables|Default|GetLevel))) true true "(R=0.000000,G=0.000000,B=0.000000,A=1.000000)" 0.0))))