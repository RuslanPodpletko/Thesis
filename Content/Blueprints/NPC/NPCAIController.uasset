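; AI controller for NPC characters that tracks an alarm target and manages the NPC's control components.
; On possession it initializes every MainNPCControlComponent and binds to the NPC's alarm, disalarm and death events, plus an empty follow-destination handler.
; When alarmed it stores the instigator and watches a SurvivalCharacter target's death to disalarm the NPC.
; Disalarm clears the target and stops components; NPC death also destroys the controller.
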(event `self.OnPossess`
  (params (PossessedPawn :type "Pawn Object Reference"))
  (`self.Init`))

(fn `BindEvents`
  (add `/Game/Blueprints/NPC/NPCCharacter.NPCAlarmed` (`self.NPC`) (`|CreateDelegate` :!event `NPCAlarmed`))
  (add `/Game/Blueprints/NPC/NPCCharacter.NPCDisAlarmed` (`self.NPC`) (`|CreateDelegate` :!event `NPCDisAlarmed`))
  (add `/Game/Blueprints/Characters/SurvivalCharacter.CharDead` (`self.NPC`) (`|CreateDelegate` :!event `Dead`))
  (add `/Game/Blueprints/NPC/Components/NPC-FollowComponent.DestReached` (`self.NPC-FollowComponent`) (`|CreateDelegate` :!event `FollowDestReached`)))

(fn `Dead`
  (params (Character :type "/Game/Blueprints/Characters/SurvivalCharacter Object Reference"))
  (`self.StopAllActions`)
  (set `self.AlarmTarget` null)
  (`self.K2_DestroyActor`))

(fn `FollowDestReached`)

(fn `Init`
  (bind _asnpccharacter (cast `/Game/Blueprints/NPC/NPCCharacter` (`self.K2_GetPawn`)))
  (set `self.NPC` _asnpccharacter)
  (for _array_element (`self.K2_GetComponentsByClass` "/Game/Blueprints/NPC/Components/MainNPCControlComponent.MainNPCControlComponent_C")
    (`/Game/Blueprints/NPC/Components/MainNPCControlComponent.Init` _array_element))
  (`self.BindEvents`))

(fn `NPCAlarmed`
  (params (Instigator :type "Pawn Object Reference"))
  (bind _output_get (set `self.AlarmTarget` Instigator))
  (bind _assurvival_character (cast `/Game/Blueprints/Characters/SurvivalCharacter` _output_get))
  (add `/Game/Blueprints/Characters/SurvivalCharacter.CharDead` _assurvival_character (`|CreateDelegate` :!event `TargetDead`))
  (`KismetSystemLibrary.PrintString` "NPC ALARMED"))

(fn `NPCDisAlarmed`
  (`|ExecutionSequence`
    (:`then_0`
      (bind _assurvival_character (cast `/Game/Blueprints/Characters/SurvivalCharacter` (`self.AlarmTarget`)))
      (remove `/Game/Blueprints/Characters/SurvivalCharacter.CharDead` _assurvival_character (`|CreateDelegate` :!event `TargetDead`)))
    (:`then_1`
      (set `self.AlarmTarget` null)
      (`self.StopAllActions`))))

(fn `StopAllActions`
  (returns (Stopped :type Boolean))
  (set `self.AlarmTarget` null)
  (`/Game/Blueprints/NPC/Components/MainNPCControlComponent.Stop` (`self.K2_GetComponentsByClass` "/Game/Blueprints/NPC/Components/MainNPCControlComponent.MainNPCControlComponent_C"))
  (return true))

(fn `TargetDead`
  (params (Character :type "/Game/Blueprints/Characters/SurvivalCharacter Object Reference"))
  (`/Game/Blueprints/NPC/NPCCharacter.DisAlarm` (`self.NPC`)))

(fn `UserConstructionScript`)