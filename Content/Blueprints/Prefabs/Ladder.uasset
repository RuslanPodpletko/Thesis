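; Climbable ladder prefab that puts a SurvivalCharacter into climbing mode while it overlaps the ladder's Box.
; Begin overlap sets the Climbing flag, switches movement to Flying and opens a Tick gate that keeps the character facing opposite the ladder's forward vector.
; End overlap, or the character hitting another actor, restores Walking and closes the gate, reusing the end-overlap cast result.
; Interact is a stub that reports failure.
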(event `self.ReceiveTick`
  (params (DeltaSeconds :type "Float (single-precision)"))
  (`/Engine/EditorBlueprintResources/StandardMacros.Gate` true :!label _label
    (:`Exit`
      (`self.SetActorRotation` (stale `self.Box.OnComponentBeginOverlap` _assurvival_character) (`KismetMathLibrary.Conv_VectorToRotator` (* (`self.GetActorForwardVector`) -1))))))

(event `self.Box.OnComponentBeginOverlap`
  (params (OtherActor :type "Actor Object Reference") (OtherComp :type "PrimitiveComponent Object Reference") (OtherBodyIndex :type Integer) (bFromSweep :type Boolean) (SweepResult :type "HitResult Structure (by ref)"))
  (bind _assurvival_character (cast `/Game/Blueprints/Characters/SurvivalCharacter` OtherActor))
  (add `self.OnActorHit` _assurvival_character (delegate `OnActorHit_Event_0`))
  (set `/Game/Blueprints/Characters/SurvivalCharacter.Climbing` true _assurvival_character)
  (`CharacterMovementComponent.SetMovementMode` (`Character.CharacterMovement` _assurvival_character) "MOVE_Flying" 0)
  (goto _label :!via `Open`))

(event `self.Box.OnComponentEndOverlap`
  (params (OtherActor :type "Actor Object Reference") (OtherComp :type "PrimitiveComponent Object Reference") (OtherBodyIndex :type Integer))
  (bind _assurvival_character (cast `/Game/Blueprints/Characters/SurvivalCharacter` OtherActor))
  (set `/Game/Blueprints/Characters/SurvivalCharacter.Climbing` false _assurvival_character :!label _label_2)
  (`CharacterMovementComponent.SetMovementMode` (`Character.CharacterMovement` _assurvival_character) "MOVE_Walking" 0)
  (goto _label :!via `Close`))

(event `OnActorHit_Event_0` :!signature `self.OnActorHit`
  (params (SelfActor :type "Actor Object Reference") (OtherActor :type "Actor Object Reference") (NormalImpulse :type "Vector Structure") (Hit :type "HitResult Structure (by ref)"))
  (if (!= OtherActor self)
    (goto _label_2)))

(fn `Interact`
  (params (Character :type "/Game/Blueprints/Characters/SurvivalCharacter Object Reference"))
  (returns (Successfull :type Boolean) (Message :type String))
  (return false ""))

(fn `UserConstructionScript`)