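; Player building component that lets a survival character preview, rotate and place constructions paid for with stored items.
; Enabling placement spawns a preview actor if StorageComponent holds the class's required Resources.
; Tick moves the preview to the location it derives from the player's interaction trace.
; Finishing removes resources, commits the actor and spawns another preview for repeat building, or cancels placement if removal fails.
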(event `self.ReceiveBeginPlay`
  (bind _assurvival_character_player (cast `/Game/Blueprints/Characters/SurvivalCharacter_Player` (`self.GetOwner`)))
  (set `self.Player` _assurvival_character_player))

(event `self.ReceiveTick`
  (params (DeltaSeconds :type "Float (single-precision)"))
  (`self.MoveConstruction`))

(fn `CheckResources`
  (params (Construction :type "/Game/Blueprints/Constructions/Constuction Class Reference"))
  (returns (HasResources :type Boolean))
  (locals (L_Item :type "/Game/Blueprints/Storage/Items/StorageItem Object Reference"))
  (for _array_element (defaults `/Game/Blueprints/Characters/BuildComponent` Construction)
    (bind (_item _count) (break `/Game/Blueprints/Storage/St_ClassItemInfo` _array_element))
    (bind _output_get (set `local.L_Item` (`.Item` (`/Game/Blueprints/Storage/StorageComponent.GetItemInStorageByClass` (`/Game/Blueprints/Characters/SurvivalCharacter.StorageComponent` (`self.Player`)) _item))))
    (`/Engine/EditorBlueprintResources/StandardMacros.IsValid` _output_get
      (:`Is Valid`
        (if (< (`/Game/Blueprints/Storage/Items/StorageItem.Count` _output_get) _count)
          (return false)))
      (:`Is Not Valid`
        (return false))))
  (return true))

(fn `FinishSetConstruction`
  (returns (Set :type Boolean))
  (`/Engine/EditorBlueprintResources/StandardMacros.IsValid` (`self.ConstructionPlacing`)
    (:`Is Valid`
      (bind _removed (`self.RemoveResources` (`self.ConstructionPlacing`)))
      (if _removed
        (`/Game/Blueprints/Constructions/Constuction.TogglePlacement` (`self.ConstructionPlacing`) false)
        (set `self.ConstructionPlacing` null)
        (`self.SpawnConstruction`)
        (return true)
        (else
          (`self.ToggleConstructionPlacement` false))))
    (:`Is Not Valid`
      (return false))))

(fn `MoveConstruction`
  (bind _constructionplacing (`self.ConstructionPlacing`))
  (`/Engine/EditorBlueprintResources/StandardMacros.IsValid` (`self.ConstructionPlacing`)
    (:`Is Valid`
      (`Actor.K2_SetActorLocation` _constructionplacing (`/Game/Blueprints/Constructions/Constuction.GetPlacementLocation` _constructionplacing (`/Game/Blueprints/Characters/SurvivalCharacter.GetInteractionInfo` (`self.Player`) (`self.MaxPlaceDistance`))) false false))))

(fn `RemoveResources`
  (params (Construcion :type "/Game/Blueprints/Constructions/Constuction Object Reference"))
  (returns (Removed :type Boolean))
  (locals (L_Item :type "/Game/Blueprints/Storage/Items/StorageItem Object Reference"))
  (for _array_element (`/Game/Blueprints/Constructions/Constuction.Resources` Construcion)
    (bind (_item _count) (break `/Game/Blueprints/Storage/St_ClassItemInfo` _array_element))
    (bind (_wasfound _item_2) (`/Game/Blueprints/Storage/StorageComponent.GetItemInStorageByClass` (`/Game/Blueprints/Characters/SurvivalCharacter.StorageComponent` (`self.Player`)) _item))
    (bind _output_get (set `local.L_Item` _item_2))
    (`/Engine/EditorBlueprintResources/StandardMacros.IsValid` _output_get
      (:`Is Valid`
        (`/Game/Blueprints/Storage/Items/StorageItem.RemoveItem` _item_2 _count))
      (:`Is Not Valid`
        (return false))))
  (return true))

(fn `RotateConstruction`
  (params (Right :type Boolean))
  (returns (Rotated :type Boolean))
  (`/Engine/EditorBlueprintResources/StandardMacros.IsValid` (`self.ConstructionPlacing`)
    (:`Is Valid`
      (`/Game/Blueprints/Constructions/Constuction.RotateConstruction` (`self.ConstructionPlacing`) Right)
      (return true))))

(fn `SpawnConstruction`
  (returns (Spawned :type Boolean))
  (`/Engine/EditorBlueprintResources/StandardMacros.IsValid` (`self.ConstructionPlacing`)
    (:`Is Not Valid`
      (if (`self.CheckResources` (`self.PlacingConstructions`))
        (bind _returnvalue (`|SpawnActorFromClass` (`self.PlacingConstructions`) (`KismetMathLibrary.MakeTransform` (`.Location` (`GameplayStatics.BreakHitResult` (`/Game/Blueprints/Characters/SurvivalCharacter.GetInteractionInfo` (`self.Player`) (`self.MaxPlaceDistance`))))) "Undefined" "OverrideRootScale" (`self.Player`)))
        (bind _output_get (set `self.ConstructionPlacing` _returnvalue))
        (`/Game/Blueprints/Constructions/Constuction.TogglePlacement` _output_get true)
        (return true)
        (else
          (return true))))))

(fn `ToggleConstructionPlacement`
  (params (Enable :type Boolean) (ConstructionClass :type "/Game/Blueprints/Constructions/Constuction Class Reference"))
  (bind _constructionplacing (`self.ConstructionPlacing`))
  (if Enable
    (set `self.PlacingConstructions` ConstructionClass)
    (`self.SpawnConstruction`)
    (else
      (set `self.PlacingConstructions` null)
      (`/Engine/EditorBlueprintResources/StandardMacros.IsValid` _constructionplacing
        (:`Is Valid`
          (`Actor.K2_DestroyActor` _constructionplacing)
          (set `self.ConstructionPlacing` null))))))