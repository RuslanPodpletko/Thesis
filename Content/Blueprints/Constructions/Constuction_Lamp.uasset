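; Interactable ceiling lamp construction that a character can switch on and off.
; The construction script runs the parent's setup, creates a dynamic lit-lamp material on the mesh and applies the initial LampEnabled state.
; Interact calls ToggleLamp, which flips that state, updating point light visibility and the material's Glow parameter together, then reports success.
; ToggleInteractAttempt always returns false.
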(fn `Interact`
  (params (Character :type "/Game/Blueprints/Characters/SurvivalCharacter Object Reference"))
  (returns (Successfull :type Boolean) (Message :type String))
  (`self.ToggleLamp`)
  (return true ""))

(fn `ToggleInteractAttempt`
  (params (Enable :type Boolean) (Character :type "/Game/Blueprints/Characters/SurvivalCharacter Object Reference") (Hit :type "HitResult Structure"))
  (returns (ReturnValue :type Boolean))
  (return false))

(fn `ToggleLamp`
  (set `self.LampEnabled` (not (`self.LampEnabled`)))
  (`SceneComponent.SetVisibility` (`self.PointLight`) (`self.LampEnabled`) false)
  (`MaterialInstanceDynamic.SetScalarParameterValue` (`self.LampDynamMat`) "Glow" (`KismetMathLibrary.SelectFloat` 1.0 0.0 (`self.LampEnabled`))))

(fn `UserConstructionScript`
  (`parent.UserConstructionScript`)
  (bind _returnvalue (`PrimitiveComponent.CreateDynamicMaterialInstance` (`self.SM_Lamp_Ceiling`) 0 "/Game/Assets/StarterContent/Props/Materials/M_LampLit.M_LampLit"))
  (bind _output_get (set `self.LampDynamMat` _returnvalue))
  (`MaterialInstanceDynamic.SetScalarParameterValue` _output_get "Glow" (`KismetMathLibrary.SelectFloat` 1.0 0.0 (`self.LampEnabled`)))
  (`SceneComponent.SetVisibility` (`self.PointLight`) (`self.LampEnabled`) false))