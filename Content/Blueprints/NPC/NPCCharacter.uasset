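; NPC character that can attack with its weapon, be alarmed and, once dead, be looted by the player.
; Damage from the player alarms it and nearby NPCs whose class matches its friend list.
; Alarm and DisAlarm switch between sprinting and walking speed and notify listeners, while a helper smoothly turns actor and controller yaw toward a direction.
; Interacting with the corpse opens the survival controller's exchange widget on its storage component.
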(event `self.ReceiveAnyDamage`
  (params (Damage :type "Float (single-precision)") (DamageType :type "DamageType Object Reference") (InstigatedBy :type "Controller Object Reference") (DamageCauser :type "Actor Object Reference"))
  (bind _returnvalue (`GameplayStatics.GetPlayerCharacter` 0))
  ;[1 1 1] Alarm by damage
  (`parent.ReceiveAnyDamage` Damage DamageType InstigatedBy DamageCauser)
  (if (== InstigatedBy (`GameplayStatics.GetPlayerController` 0))
    (`self.Alarm` _returnvalue)
    (`self.AlarmFriends` _returnvalue)))

(event `Attack`
  (params (Target :type "Actor Object Reference") (AsMelee :type Boolean))
  (set `self.Attacking` true)
  (`self.ShootFromWeapon` true AsMelee))

(event `StopAttack`
  (set `self.Attacking` false)
  (`self.ShootFromWeapon` false))

(fn `Alarm`
  (params (Instigator :type "Pawn Object Reference"))
  (if (and (not (`self.Alarmed`)) (not (`self.Dead`)))
    (set `self.Alarmed` true)
    (set `CharacterMovementComponent.MaxWalkSpeed` (`self.SprintingSpeed`) (`self.CharacterMovement`))
    (set `self.Sprinting` true)
    (`self.NPCAlarmed` Instigator)))

(fn `AlarmFriends`
  (params (Instigator :type "Pawn Object Reference"))
  (bind _outactors (`GameplayStatics.GetAllActorsOfClass` "NPCCharacter_C"))
  (for _array_element _outactors
    (if (< (`KismetMathLibrary.VSize` (- (`self.K2_GetActorLocation` _array_element) (`self.K2_GetActorLocation`))) (`self.AlarmFriendsRadius`))
      (if (!= _array_element self)
        (if (`self.IsFriend` _array_element)
          (`self.Alarm` _array_element Instigator))))))

(fn `DisAlarm`
  (set `self.Alarmed` false)
  (set `CharacterMovementComponent.MaxWalkSpeed` (`self.WalkingSpeed`) (`self.CharacterMovement`))
  (set `self.Sprinting` false)
  (`self.NPCDisAlarmed`))

(fn `Interact`
  (params (Character :type "/Game/Blueprints/Characters/SurvivalCharacter Object Reference"))
  (returns (Successfull :type Boolean) (Message :type String))
  (if (`self.Dead`)
    (bind _assurvival_player_controller (cast `/Game/Blueprints/Gamemode/SurvivalPlayerController` (`self.GetController` Character))
      (:`then`
        (`/Game/Blueprints/Gamemode/SurvivalPlayerController.ExchangeWidget` _assurvival_player_controller (`self.StorageComponent`) false)
        (return true ""))
      (:`CastFailed`
        (return false "")))
    (else
      (return false "Not Dead"))))

(fn `IsFriend`
  (params (Pawn :type "Pawn Object Reference"))
  (returns (Friend :type Boolean))
  (bind _returnvalue (`GameplayStatics.GetObjectClass` Pawn))
  (for _array_element (`self.FriendList`)
    (if (or (`KismetMathLibrary.ClassIsChildOf` _returnvalue _array_element) (== _array_element _returnvalue))
      (return true)))
  (return false))

(fn `RotateTowardDirection`
  (params (Direction :type "Vector Structure") (DeltaTime :type "Float (double-precision)") (InterpSpeed :type "Float (double-precision)") (RotatedThreshold :type "Float (double-precision)"))
  (returns (Rotated :type Boolean))
  (bind (_returnvalue_roll _returnvalue_pitch _returnvalue_yaw) (`KismetMathLibrary.BreakRotator` (`self.K2_GetActorRotation`)))
  (bind _returnvalue (`self.GetController`))
  (bind _yaw (.yaw (`KismetMathLibrary.Conv_VectorToRotator` Direction)))
  (`self.K2_SetActorRotation` (`KismetMathLibrary.RInterpTo_Constant` (`self.K2_GetActorRotation`) (`KismetMathLibrary.MakeRotator` 0.0 0.0 _yaw) DeltaTime InterpSpeed))
  (`Controller.SetControlRotation` _returnvalue (`KismetMathLibrary.MakeRotator` (.roll (`Controller.GetControlRotation` _returnvalue)) (.pitch (`Controller.GetControlRotation` _returnvalue)) (.yaw (`self.K2_GetActorRotation`))))
  (return (`KismetMathLibrary.InRange_FloatFloat` _returnvalue_yaw (- _yaw RotatedThreshold) (+ _yaw RotatedThreshold))))

(fn `ToggleInteractAttempt`
  (params (Enable :type Boolean) (Character :type "/Game/Blueprints/Characters/SurvivalCharacter Object Reference") (Hit :type "HitResult Structure"))
  (returns (ReturnValue :type Boolean))
  (return false))

(fn `UserConstructionScript`
  (`parent.UserConstructionScript`))