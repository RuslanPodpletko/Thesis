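; Placeable wall piece for a building system that can hold a door or window.
; Placement snaps to foundation tops in 90-degree yaw steps, or to the closest wall within range, using dot products to choose corner or neighbour offsets.
; Setting a door or window swaps the full wall for upper and lower segments, toggling collision; destroying the insert restores it.
; Breaking the wall also breaks its door and window.
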(event `self.BreakConstruction`
  (`parent.BreakConstruction`)
  (`|ExecutionSequence`
    (:`then_0`
      (`/Engine/EditorBlueprintResources/StandardMacros.IsValid` (`self.Door`)
        (:`Is Valid`
          (`self.BreakConstruction` (`self.Door`)))))
    (:`then_1`
      (`/Engine/EditorBlueprintResources/StandardMacros.IsValid` (`self.Window`)
        (:`Is Valid`
          (`self.BreakConstruction` (`self.Window`)))))))

(fn `ConstructionDestroyed`
  (params (Construction :type "Actor Object Reference"))
  (set `self.Door` null)
  (set `self.Window` null)
  (`SceneComponent.SetVisibility` (`self.Up`) false false)
  (`SceneComponent.SetVisibility` (`self.Down`) false false)
  (`SceneComponent.SetVisibility` (`self.Wall`) true false)
  (`PrimitiveComponent.SetCollisionEnabled` (`self.Wall`) "QueryOnly")
  (`PrimitiveComponent.SetCollisionEnabled` (`self.Up`) "NoCollision")
  (`PrimitiveComponent.SetCollisionEnabled` (`self.Down`) "NoCollision"))

(fn `GetPlacementLocation`
  (params (LookAtHit :type "HitResult Structure"))
  (returns (Location :type "Vector Structure"))
  (locals (L_Distance :type "Float (double-precision)" :default 160.0) (L_ClosesWall :type "/Game/Blueprints/Constructions/Constuction_Wall Object Reference") (L_Hit :type "HitResult Structure"))
  (bind (_bblockinghit _binitialoverlap _time _location) (`GameplayStatics.BreakHitResult` (`local.L_Hit`)))
  (bind (_bblockinghit_2 _binitialoverlap_2 _time_2 _location_2 _impactpoint _normal _impactnormal _physmat _hitactor) (`GameplayStatics.BreakHitResult` (`local.L_Hit`)))
  (bind _returnvalue (`self.GetActorForwardVector` (`local.L_ClosesWall`)))
  (bind _returnvalue_2 (`self.GetActorRightVector` (`local.L_ClosesWall`)))
  (bind _returnvalue_3 (`self.GetActorForwardVector` (`local.L_ClosesWall`)))
  (bind (_origin _boxextent) (`self.GetActorBounds` _hitactor false))
  (bind _returnvalue_4 (`KismetMathLibrary.GetDirectionUnitVector` (`self.K2_GetActorLocation` (`local.L_ClosesWall`)) _location))
  (set `local.L_Hit` LookAtHit)
  (cast `/Game/Blueprints/Constructions/Constuction_Fundament` (`.HitActor` (`GameplayStatics.BreakHitResult` (`local.L_Hit`)))
    (:`then`
      (return (+ (+ _origin (* _boxextent (0.0 0.0 1.0))) (`KismetMathLibrary.RotateAngleAxis` (40.0 0.0 0.0) (* (`KismetMathLibrary.Round` (/ (.yaw (`KismetMathLibrary.FindLookAtRotation` (`self.K2_GetActorLocation` _hitactor) _location_2)) 90.0)) 90.0) (0.0 0.0 1.0)))))
    (:`CastFailed`
      (bind _outactors (`GameplayStatics.GetAllActorsOfClass` "Constuction_Wall_C"))
      (for _array_element _outactors
        (if (!= self _array_element)
          (bind _returnvalue_5 (`KismetMathLibrary.VSize` (- (`self.K2_GetActorLocation` _array_element) (`.Location` (`GameplayStatics.BreakHitResult` (`local.L_Hit`))))))
          (if (<= _returnvalue_5 150.0)
            (if (<= _returnvalue_5 (`local.L_Distance`))
              (set `local.L_Distance` _returnvalue_5)
              (set `local.L_ClosesWall` _array_element)))))
      (`/Engine/EditorBlueprintResources/StandardMacros.IsValid` (`local.L_ClosesWall`)
        (:`Is Valid`
          (return (`KismetMathLibrary.SelectVector` (+ (`self.K2_GetActorLocation` (`local.L_ClosesWall`)) (`KismetMathLibrary.SelectVector` (* _returnvalue 50.0) (* _returnvalue -50.0) (> (`KismetMathLibrary.Dot_VectorVector` _returnvalue _returnvalue_4) 0.0)) (`KismetMathLibrary.SelectVector` (* _returnvalue_2 50.0) (* _returnvalue_2 -50.0) (> (`KismetMathLibrary.Dot_VectorVector` _returnvalue_4 _returnvalue_2) 0.0))) (+ (`self.K2_GetActorLocation` (`local.L_ClosesWall`)) (`KismetMathLibrary.SelectVector` (* _returnvalue_3 100.0) (* _returnvalue_3 -100.0) (> (`KismetMathLibrary.Dot_VectorVector` _returnvalue_3 (`KismetMathLibrary.GetDirectionUnitVector` (`self.K2_GetActorLocation` (`local.L_ClosesWall`)) _location)) 0.0))) (`KismetMathLibrary.InRange_FloatFloat` (`KismetMathLibrary.Dot_VectorVector` (`self.GetActorForwardVector` (`local.L_ClosesWall`)) (`self.GetActorForwardVector`)) -0.01 0.01))))
        (:`Is Not Valid`
          (return _location))))))

(fn `SetDoor`
  (params (Door :type "/Game/Blueprints/Constructions/Constuction_Door Object Reference"))
  (bind _output_get (set `self.Door` Door))
  (`/Engine/EditorBlueprintResources/StandardMacros.IsValid` _output_get
    (:`Is Valid`
      (`SceneComponent.SetVisibility` (`self.Up`) true false)
      (`SceneComponent.SetVisibility` (`self.Wall`) false false)
      (`SceneComponent.SetVisibility` (`self.Down`) false false)
      (`PrimitiveComponent.SetCollisionEnabled` (`self.Wall`) "NoCollision")
      (`PrimitiveComponent.SetCollisionEnabled` (`self.Down`) "NoCollision")
      (`PrimitiveComponent.SetCollisionEnabled` (`self.Up`) "QueryOnly")
      (add `self.OnDestroyed` (`self.Door`) (`|CreateDelegate` :!event `ConstructionDestroyed`)))
    (:`Is Not Valid`
      (`SceneComponent.SetVisibility` (`self.Up`) false false)
      (`SceneComponent.SetVisibility` (`self.Down`) false false)
      (`SceneComponent.SetVisibility` (`self.Wall`) true false)
      (`PrimitiveComponent.SetCollisionEnabled` (`self.Wall`) "QueryOnly")
      (`PrimitiveComponent.SetCollisionEnabled` (`self.Up`) "NoCollision")
      (`PrimitiveComponent.SetCollisionEnabled` (`self.Down`) "NoCollision"))))

(fn `SetWindow`
  (params (Window :type "/Game/Blueprints/Constructions/Constuction_Window Object Reference"))
  (bind _output_get (set `self.Window` Window))
  (`/Engine/EditorBlueprintResources/StandardMacros.IsValid` _output_get
    (:`Is Valid`
      (`SceneComponent.SetVisibility` (`self.Up`) true false)
      (`SceneComponent.SetVisibility` (`self.Down`) true false)
      (`SceneComponent.SetVisibility` (`self.Wall`) false false)
      (`PrimitiveComponent.SetCollisionEnabled` (`self.Wall`) "NoCollision")
      (`PrimitiveComponent.SetCollisionEnabled` (`self.Up`) "QueryOnly")
      (`PrimitiveComponent.SetCollisionEnabled` (`self.Down`) "QueryOnly")
      (add `self.OnDestroyed` (`self.Window`) (`|CreateDelegate` :!event `ConstructionDestroyed`)))
    (:`Is Not Valid`
      (`SceneComponent.SetVisibility` (`self.Up`) false false)
      (`SceneComponent.SetVisibility` (`self.Down`) false false)
      (`SceneComponent.SetVisibility` (`self.Wall`) true false)
      (`PrimitiveComponent.SetCollisionEnabled` (`self.Wall`) "QueryOnly")
      (`PrimitiveComponent.SetCollisionEnabled` (`self.Up`) "NoCollision")
      (`PrimitiveComponent.SetCollisionEnabled` (`self.Down`) "NoCollision"))))

(fn `UserConstructionScript`
  (`parent.UserConstructionScript`)
  (`|ExecutionSequence`
    (:`then_0`
      (`/Engine/EditorBlueprintResources/StandardMacros.IsValid` (`self.Door`)
        (:`Is Valid`
          (`self.SetDoor` (`self.Door`)))))
    (:`then_1`
      (`/Engine/EditorBlueprintResources/StandardMacros.IsValid` (`self.Window`)
        (:`Is Valid`
          (`self.SetWindow` (`self.Window`)))))))