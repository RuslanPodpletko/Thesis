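; Buildable door construction that snaps into wall pieces during placement and opens or closes when the player interacts.
; While placing, Tick traces from the player, releases the previous wall and claims a looked-at wall without a window or door, matching its rotation.
; Placement location follows that wall, or a far-off point when none is held.
; Interacting toggles a timeline that swings the door mesh 90 degrees.
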(event `self.ReceiveTick`
  (params (DeltaSeconds :type "Float (single-precision)"))
  (bind _lookatwall (`self.LookAtWall`))
  (if (`self.Placing`)
    (bind _assurvival_character_player (cast `/Game/Blueprints/Characters/SurvivalCharacter_Player` (`GameplayStatics.GetPlayerCharacter` 0)))
    (bind (_bblockinghit _binitialoverlap _time _location _impactpoint _normal _impactnormal _physmat _hitactor) (`GameplayStatics.BreakHitResult` (`/Game/Blueprints/Characters/SurvivalCharacter.GetInteractionInfo` _assurvival_character_player 2000.0)))
    (if (not (== (`self.LookAtWall`) _hitactor))
      (`/Engine/EditorBlueprintResources/StandardMacros.IsValid` _lookatwall
        (:`Is Valid`
          (`/Game/Blueprints/Constructions/Constuction_Wall.SetDoor` _lookatwall null)
          (set `self.LookAtWall` null))
        (:`Is Not Valid`
          _))
      (bind _asconstuction_wall (cast `/Game/Blueprints/Constructions/Constuction_Wall` _hitactor))
      (if (not (or (`KismetSystemLibrary.IsValid` (`/Game/Blueprints/Constructions/Constuction_Wall.Window` _asconstuction_wall)) (`KismetSystemLibrary.IsValid` (`/Game/Blueprints/Constructions/Constuction_Wall.Door` _asconstuction_wall))))
        (bind _output_get (set `self.LookAtWall` _asconstuction_wall))
        (`self.K2_SetActorRotation` (`self.K2_GetActorRotation` _output_get))
        (`/Game/Blueprints/Constructions/Constuction_Wall.SetDoor` (`self.LookAtWall`) self)))))

(event `OpenCloseDoor`
  (bind _output_get (set `self.Opened` (not (`self.Opened`))))
  (if _output_get
    (bind (_direction _lerp) (`Timeline|DoorAnimation` :!label _label)
      (:`Update`
        (`SceneComponent.K2_SetRelativeRotation` (`self.Door`) (`KismetMathLibrary.RLerp` (struct) (struct :`Yaw` 90.0) _lerp) false false)))
    (else
      (goto _label :!via `Reverse`))))

(fn `GetPlacementLocation`
  (params (LookAtHit :type "HitResult Structure"))
  (returns (Location :type "Vector Structure"))
  (locals (L_Distance :type "Float (double-precision)" :default 160.0) (L_ClosesWall :type "/Game/Blueprints/Constructions/Constuction_Wall Object Reference"))
  (`/Engine/EditorBlueprintResources/StandardMacros.IsValid` (`self.LookAtWall`)
    (:`Is Valid`
      (return (`self.K2_GetActorLocation` (`self.LookAtWall`))))
    (:`Is Not Valid`
      (return (-99999.0 -9999.0 -9999.0)))))

(fn `Interact`
  (params (Character :type "/Game/Blueprints/Characters/SurvivalCharacter Object Reference"))
  (returns (Successfull :type Boolean) (Message :type String))
  (`self.OpenCloseDoor`)
  (return true ""))

(fn `ToggleInteractAttempt`
  (params (Enable :type Boolean) (Character :type "/Game/Blueprints/Characters/SurvivalCharacter Object Reference") (Hit :type "HitResult Structure"))
  (returns (ReturnValue :type Boolean))
  (return false))

(fn `UserConstructionScript`
  (`parent.UserConstructionScript`))