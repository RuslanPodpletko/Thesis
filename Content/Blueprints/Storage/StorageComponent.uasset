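; Inventory component that stores item actors in a paged grid under a maximum weight.
; Adding checks weight and the first free space fitting the item's size, then merges stackable items into a same-class stack or places them.
; Items can be moved, dropped before the owner or transferred between storages, with partial stacks spawned as new actors.
; BeginPlay spawns fixed and chance-rolled starting items; EndPlay destroys stored items.
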(event `self.ReceiveBeginPlay`
  (`self.CreateItems` (`self.BeginItems`))
  (`self.CreateItems` (`self.GenerateRandomItems`)))

(event `self.ReceiveEndPlay`
  (params (EndPlayReason :type "EEndPlayReason Enum" :default "Destroyed"))
  (`self.OnOwnerDestroyed` null))

(fn `AddItem`
  (params (Item :type "/Game/Blueprints/Storage/Items/StorageItem Object Reference"))
  (returns (Added :type Boolean) (ItemAdded :type "/Game/Blueprints/Storage/Items/StorageItem Object Reference"))
  (locals (L_Item :type "/Game/Blueprints/Storage/Items/StorageItem Object Reference") (NewLocalVar_0 :type "/Game/Blueprints/Storage/Items/StorageItem Object Reference"))
  (bind _l_item (`local.L_Item`))
  (bind _l_item_2 (`local.L_Item`))
  (bind _output_get (set `local.L_Item` Item))
  (bind (_canadd _x _y _page) (`self.CheckIfItemCanBeAdded` _output_get))
  (if _canadd
    (bind (_canbestacked _stackin) (`self.CheckItemsForStack` (`local.L_Item`)))
    (if _canbestacked
      (`self.StackItem` (`local.L_Item`) _stackin)
      (`/Game/Blueprints/Storage/Items/StorageItem.DestroyItem` (`local.L_Item`))
      (`self.InventoryUpdated`)
      (return true _stackin)
      (else
        ;[1 1 1] Add new item
        (`KismetArrayLibrary.Array_Add` (`self.Items`) _l_item)
        (`self.ChangeTotalWeight` (`/Game/Blueprints/Storage/Items/StorageItem.GetItemWeight` _l_item true 0))
        (`/Game/Blueprints/Storage/Items/StorageItem.ItemAddedToStorage` _l_item_2 self _x _y _page)
        (`self.InventoryUpdated`)
        (return true _l_item_2)))
    (else
      (return false null))))

(fn `ChangeItemLocation`
  (params (Item :type "/Game/Blueprints/Storage/Items/StorageItem Object Reference") (X :type Integer) (Y :type Integer) (Page :type Integer))
  (returns (Changed :type Boolean))
  (locals (L_Items :type "Array of /Game/Blueprints/Storage/Items/StorageItem Object Reference"))
  (bind _slotsarefree (`self.CheckSlotsForItem` Item X Y Page))
  (if _slotsarefree
    (`/Game/Blueprints/Storage/Items/StorageItem.RelocateItem` Item X Y Page)
    (`self.InventoryUpdated`)
    (return true)
    (else
      (return false))))

(fn `ChangeTotalWeight`
  (params (Value :type "Float (double-precision)"))
  (set `self.StorageTotalWeight` (+ Value (`self.StorageTotalWeight`))))

(fn `CheckFreeSlotForItem`
  (params (Item :type "/Game/Blueprints/Storage/Items/StorageItem Object Reference"))
  (returns (NoFreeSlot :type Boolean) (X :type Integer) (Y :type Integer) (Page :type Integer))
  (locals (L_Item :type "/Game/Blueprints/Storage/Items/StorageItem Object Reference") (L_Page :type Integer) (L_X :type Integer) (L_Y :type Integer) (L_SlotNotFree :type Boolean) (L_SizeX :type Integer) (L_SizeY :type Integer))
  (set `local.L_Item` Item)
  (for _index (range 1 (+ (`self.StorageSizePages`) 1))
    (set `local.L_Page` _index)
    (for _index_2 (range (`self.StorageSizeY`))
      (set `local.L_Y` _index_2)
      (for _index_3 (range (`self.StorageSizeX`))
        (set `local.L_X` _index_3)
        (bind (_item _free) (`self.CheckSlot` (`local.L_Page`) (`local.L_X`) (`local.L_Y`)))
        (if _free
          (bind _slotsarefree (`self.CheckSlotsForItem` (`local.L_Item`) (`local.L_X`) (`local.L_Y`) (`local.L_Page`)))
          (if _slotsarefree
            (return false (`local.L_X`) (`local.L_Y`) (`local.L_Page`)))))))
  (return true 0 0 0))

(fn `CheckIfItemCanBeAdded`
  (params (Item :type "/Game/Blueprints/Storage/Items/StorageItem Object Reference"))
  (returns (CanAdd :type Boolean) (X :type Integer) (Y :type Integer) (Page :type Integer))
  (locals (L_X :type Integer))
  (if (not (`self.CheckIfItemCanBeAddedByWeight` Item true))
    (bind (_nofreeslot _x _y _page) (`self.CheckFreeSlotForItem` Item))
    (if (not _nofreeslot)
      (return true _x _y _page)
      (else
        _)))
  (return false 0 0 0))

(fn `CheckIfItemCanBeAddedByWeight`
  (params (Item :type "/Game/Blueprints/Storage/Items/StorageItem Object Reference") (Total :type Boolean) (Count :type Integer))
  (returns (ReturnValue :type Boolean))
  (return (> (+ (`self.StorageTotalWeight`) (`/Game/Blueprints/Storage/Items/StorageItem.GetItemWeight` Item Total Count)) (`self.StorageMaxWeight`))))

(fn `CheckItemsForStack`
  (params (Item :type "/Game/Blueprints/Storage/Items/StorageItem Object Reference"))
  (returns (CanBeStacked :type Boolean) (StackIn :type "/Game/Blueprints/Storage/Items/StorageItem Object Reference"))
  (locals (L_ItemForStackFound :type Boolean) (L_ItemToStackIn :type "/Game/Blueprints/Storage/Items/StorageItem Object Reference"))
  (bind (_wasfound _item) (`self.GetItemInStorageByClass` (`GameplayStatics.GetObjectClass` Item)))
  (if (`/Game/Blueprints/Storage/Items/StorageItem.CanBeStacked` Item)
    (return _wasfound _item)
    (else
      (return false null))))

(fn `CheckSlot`
  (params (Page :type Integer) (X :type Integer) (Y :type Integer) (CheckExactSlot :type Boolean))
  (returns (Item :type "/Game/Blueprints/Storage/Items/StorageItem Object Reference") (Free :type Boolean))
  (locals (L_Page :type Integer) (L_X :type Integer) (L_Y :type Integer) (L_Item :type "/Game/Blueprints/Storage/Items/StorageItem Object Reference"))
  (bind _l_page (`local.L_Page`))
  (bind _l_y (`local.L_Y`))
  (bind _l_item (`local.L_Item`))
  (bind _l_x (`local.L_X`))
  (set `local.L_Page` Page)
  (set `local.L_X` X)
  (set `local.L_Y` Y)
  (`|ExecutionSequence`
    (:`then_0`
      ;[1 1 1] Check for slot outside inventory borders
      (`|ExecutionSequence`
        (:`then_0`
          (if (or (> _l_page (`self.StorageSizePages`)) (< _l_page 1))
            (return null false)))
        (:`then_1`
          (if (or (>= _l_x (`self.StorageSizeX`)) (< _l_x 0))
            (return null false)))
        (:`then_2`
          (if (or (>= _l_y (`self.StorageSizeY`)) (< _l_y 0))
            (return null false)))))
    (:`then_1`
      (for _array_element (`self.Items`)
        (bind (_x _y _page) (`/Game/Blueprints/Storage/Items/StorageItem.LocateItem` _array_element))
        (if (select `bool` CheckExactSlot :`false` (`/Game/Blueprints/Storage/Items/StorageItem.CheckIfItemIsInSlot` _array_element (`local.L_X`) (`local.L_Y`) (`local.L_Page`)) :`true` (and (== _x (`local.L_X`)) (== _y (`local.L_Y`)) (== _page (`local.L_Page`))))
          (set `local.L_Item` _array_element)
          (break))))
    (:`then_2`
      (return _l_item (not (`KismetSystemLibrary.IsValid` _l_item))))))

(fn `CheckSlotsForItem`
  (params (Item :type "/Game/Blueprints/Storage/Items/StorageItem Object Reference") (X :type Integer) (Y :type Integer) (Page :type Integer))
  (returns (SlotsAreFree :type Boolean))
  (locals (L_Item :type "/Game/Blueprints/Storage/Items/StorageItem Object Reference") (L_X :type Integer) (L_Y :type Integer) (L_Page :type Integer) (L_SizeX :type Integer) (L_SizeY :type Integer) (L_SlotNotFree :type Boolean))
  (bind (_x _y _page _sizex _sizey) (`/Game/Blueprints/Storage/Items/StorageItem.LocateItem` (`local.L_Item`)))
  (set `local.L_Item` Item)
  (set `local.L_X` X)
  (set `local.L_Y` Y)
  (set `local.L_Page` Page)
  (for _index (range _sizey)
    (set `local.L_SizeY` _index)
    (for _index_2 (range _sizex)
      (set `local.L_SizeX` _index_2)
      (bind (_item _free) (`self.CheckSlot` (`local.L_Page`) (+ (`local.L_SizeX`) (`local.L_X`)) (+ (`local.L_SizeY`) (`local.L_Y`))))
      (if (and (not _free) (!= _item (`local.L_Item`)))
        (return false))))
  (return true))

(fn `ClearInventory`
  (set `self.Items` (`|MakeArray`))
  (set `self.StorageTotalWeight` 0.0)
  (`self.InventoryUpdated`))

(fn `CreateItems`
  (params (Items :type "Array of /Game/Blueprints/Storage/St_ClassItemInfo Structure"))
  (returns (CreatedItems :type "Array of /Game/Blueprints/Storage/Items/StorageItem Object Reference"))
  (locals (L_CreatedItems :type "Array of /Game/Blueprints/Storage/Items/StorageItem Object Reference") (L_ItemInfo :type "/Game/Blueprints/Storage/St_ClassItemInfo Structure" :default (struct)))
  (bind (_item _count) (break `/Game/Blueprints/Storage/St_ClassItemInfo` (`local.L_ItemInfo`)))
  (for _array_element Items
    (set `local.L_ItemInfo` _array_element)
    (if (`.CanBeStacked` (defaults `/Game/Blueprints/Storage/StorageComponent` (`.Item_7_27EAD8B9441E0C560BC7C2A876472EC1` (break `/Game/Blueprints/Storage/St_ClassItemInfo` _array_element))))
      (bind _returnvalue (`|SpawnActorFromClass` (`.Item_7_27EAD8B9441E0C560BC7C2A876472EC1` (break `/Game/Blueprints/Storage/St_ClassItemInfo` (`local.L_ItemInfo`))) (`KismetMathLibrary.MakeTransform` (0.0 0.0 0.0)) "AlwaysSpawn" "OverrideRootScale" null (`KismetMathLibrary.SelectInt` _count 1 (`.CanBeStacked` (defaults `/Game/Blueprints/Storage/StorageComponent` _item))) :!label _label))
      (bind (_added _itemadded) (`self.AddItem` _returnvalue))
      (if _added
        (`KismetArrayLibrary.Array_Add` (`local.L_CreatedItems`) _itemadded)
        (else
          (`KismetArrayLibrary.Array_RemoveItem` (`local.L_CreatedItems`) _returnvalue)
          (`/Game/Blueprints/Storage/Items/StorageItem.DestroyItem` _returnvalue)))
      (else
        (for _ (range 1 (+ _count 1))
          (goto _label)))))
  (return (`local.L_CreatedItems`)))

(fn `DropItemToWorld`
  (params (Item :type "/Game/Blueprints/Storage/Items/StorageItem Object Reference") (DropAll :type Boolean) (Count :type Integer))
  (locals (L_Item :type "/Game/Blueprints/Storage/Items/StorageItem Object Reference") (L_Count :type Integer))
  (set `local.L_Item` Item)
  (if DropAll
    ;[1 1 1] Drop all
    (bind _removed (`self.RemoveItem` (`local.L_Item`) 0 true :!label _label))
    (if _removed
      (`/Game/Blueprints/Storage/Items/StorageItem.DroppedToWorld` (`local.L_Item`) (`self.DropLocation`)))
    (else
      (bind _output_get (set `local.L_Count` Count))
      (if (`self.IsFullStackByCount` (`local.L_Item`) _output_get)
        (goto _label)
        (else
          ;[1 1 1] Drop some
          (bind _removed_2 (`self.RemoveItem` (`local.L_Item`) (`local.L_Count`)))
          (if _removed_2
            (bind _returnvalue (`|SpawnActorFromClass` (`GameplayStatics.GetObjectClass` (`local.L_Item`)) (`KismetMathLibrary.MakeTransform` (0.0 0.0 0.0)) "AlwaysSpawn" "OverrideRootScale" null (`local.L_Count`)))
            (`/Game/Blueprints/Storage/Items/StorageItem.FreezePhysComponents` _returnvalue true)
            (`/Game/Blueprints/Storage/Items/StorageItem.DroppedToWorld` _returnvalue (`self.DropLocation`))))))))

(fn `DropLocation`
  (returns (ReturnValue :type "Vector Structure"))
  (bind _returnvalue (`self.GetOwner`))
  ;[1 1 1] Drop location
  (return (+ (`Actor.K2_GetActorLocation` _returnvalue) (* (`Actor.GetActorForwardVector` _returnvalue) (`self.DropDistance`)))))

(fn `GenerateRandomItems`
  (returns (Items :type "Array of /Game/Blueprints/Storage/St_ClassItemInfo Structure"))
  (locals (L_GeneratedItems :type "Array of /Game/Blueprints/Storage/St_ClassItemInfo Structure"))
  (for _array_element (`self.RandomBeginItems`)
    (bind (_iteminfo _chance) (break `/Game/Blueprints/Storage/St_RandomItem` _array_element))
    (if (>= _chance (`KismetMathLibrary.RandomFloatInRange` 0.0 100.0))
      (`KismetArrayLibrary.Array_Add` (`local.L_GeneratedItems`) _iteminfo)))
  (return (`local.L_GeneratedItems`)))

(fn `GetItemInStorageByClass`
  (params (Class :type "/Game/Blueprints/Storage/Items/StorageItem Class Reference"))
  (returns (WasFound :type Boolean) (Item :type "/Game/Blueprints/Storage/Items/StorageItem Object Reference"))
  (for _array_element (`self.Items`)
    (if (== (`GameplayStatics.GetObjectClass` _array_element) Class)
      (return true _array_element)))
  (return false null))

(fn `GetItems`
  (returns (Items :type "Array of /Game/Blueprints/Storage/Items/StorageItem Object Reference"))
  (return (`self.Items`)))

(fn `GetWeight`
  (returns (Total :type "Float (double-precision)") (Max :type "Float (double-precision)"))
  (return (`self.StorageTotalWeight`) (`self.StorageMaxWeight`)))

(fn `IsFullStackByCount`
  (params (Item :type "/Game/Blueprints/Storage/Items/StorageItem Object Reference") (Count :type Integer))
  (returns (FullStack :type Boolean) (Remain :type Integer))
  (bind _returnvalue (- (`/Game/Blueprints/Storage/Items/StorageItem.Count` Item) Count))
  (return (<= _returnvalue 0) _returnvalue))

(fn `OnOwnerDestroyed`
  (params (Owner :type "Actor Object Reference"))
  (for _array_element (`self.Items`)
    (`/Game/Blueprints/Storage/Items/StorageItem.DestroyItem` _array_element)
    (`KismetSystemLibrary.PrintString` (`KismetSystemLibrary.GetDisplayName` _array_element) true true (struct :`R` 0.200081 :`G` 0.229 :`B` 0.38 :`A` 1.0))))

(fn `PlaceToAnotherStorage`
  (params (Item :type "/Game/Blueprints/Storage/Items/StorageItem Object Reference") (Storage :type "/Game/Blueprints/Storage/StorageComponent Object Reference") (Total :type Boolean :default true) (Count :type Integer :default -1))
  (returns (Placed :type Boolean) (PlacedItem :type "/Game/Blueprints/Storage/Items/StorageItem Object Reference"))
  (locals (L_Item :type "/Game/Blueprints/Storage/Items/StorageItem Object Reference") (L_ToStorage :type "/Game/Blueprints/Storage/StorageComponent Object Reference") (L_Count :type Integer) (L_Total :type Boolean))
  (set `local.L_Item` Item)
  (set `local.L_ToStorage` Storage)
  (set `local.L_Count` Count)
  (bind _output_get (set `local.L_Total` Total))
  (if _output_get
    ;[1 1 1] Place full item
    (bind _canadd (`self.CheckIfItemCanBeAdded` (`local.L_ToStorage`) (`local.L_Item`)))
    (if _canadd
      (bind _removed (`self.RemoveItem` (`local.L_Item`) 0 true))
      (if _removed
        (bind _added (`self.AddItem` (`local.L_ToStorage`) (`local.L_Item`)))
        (if _added
          (return true (`local.L_Item`))
          (else
            _))))
    (return false null)
    (else
      ;[1 1 1] Place by count
      (bind _createditems (`self.CreateItems` (`local.L_ToStorage`) (`|MakeArray` (make `/Game/Blueprints/Storage/St_ClassItemInfo` (`GameplayStatics.GetObjectClass` (`local.L_Item`)) (`local.L_Count`)))))
      (if (>= (`KismetArrayLibrary.Array_Length` _createditems) 1)
        (`self.RemoveItem` (`local.L_Item`) (`local.L_Count`))
        (return true (`KismetArrayLibrary.Array_Get` _createditems))
        (else
          (return false null))))))

(fn `RemoveItem`
  (params (StorageItem :type "/Game/Blueprints/Storage/Items/StorageItem Object Reference") (Count :type Integer) (RemoveAll :type Boolean) (DestroyAfterLast :type Boolean))
  (returns (Removed :type Boolean))
  (locals (L_Item :type "/Game/Blueprints/Storage/Items/StorageItem Object Reference") (L_Count :type Integer))
  (bind _output_get (set `local.L_Item` StorageItem))
  (set `local.L_Count` (`KismetMathLibrary.SelectInt` (`/Game/Blueprints/Storage/Items/StorageItem.Count` _output_get) Count RemoveAll))
  (if (== (`.Storage` (`/Game/Blueprints/Storage/Items/StorageItem.IsInStorage` (`local.L_Item`))) self)
    (bind _removedall (`self.RemoveStackedItem` (`local.L_Item`) (`local.L_Count`)))
    (`self.ChangeTotalWeight` (* (`/Game/Blueprints/Storage/Items/StorageItem.GetItemWeight` (`local.L_Item`) _removedall (`local.L_Count`)) -1.0))
    (if _removedall
      (`KismetArrayLibrary.Array_RemoveItem` (`self.Items`) (`local.L_Item`))
      (`/Game/Blueprints/Storage/Items/StorageItem.ItemRemovedFromStorage` (`local.L_Item`) self)
      (`self.InventoryUpdated`)
      (if DestroyAfterLast
        (`/Game/Blueprints/Storage/Items/StorageItem.DestroyItem` (`local.L_Item`))
        (return true)
        (else
          (return true)))
      (else
        (`self.InventoryUpdated`)
        (return (> (`local.L_Count`) 0))))
    (else
      (return false))))

(fn `RemoveStackedItem`
  (params (Item :type "/Game/Blueprints/Storage/Items/StorageItem Object Reference") (Count :type Integer))
  (returns (RemovedAll :type Boolean))
  (locals (L_Item :type "/Game/Blueprints/Storage/Items/StorageItem Object Reference") (L_RemovedAll :type Boolean))
  (bind _l_item (`local.L_Item`))
  (bind _output_get (set `local.L_Item` Item))
  (bind (_fullstack _remain) (`self.IsFullStackByCount` _output_get Count))
  (bind _output_get_2 (set `local.L_RemovedAll` _fullstack))
  (if (not _output_get_2)
    (set `/Game/Blueprints/Storage/Items/StorageItem.Count` _remain _l_item))
  (`/Game/Blueprints/Storage/Items/StorageItem.ItemRemoved` _l_item _l_item Count)
  (return (`local.L_RemovedAll`)))

(fn `SetInventoryItems`
  (params (Items :type "Array of /Game/Blueprints/Storage/Items/StorageItem Object Reference"))
  (set `self.Items` Items)
  (`self.InventoryUpdated`)
  (set `self.StorageTotalWeight` 0.0)
  (for _array_element (`self.Items`)
    (`self.ChangeTotalWeight` (`/Game/Blueprints/Storage/Items/StorageItem.GetItemWeight` _array_element true 0))))

(fn `StackItem`
  (params (Item :type "/Game/Blueprints/Storage/Items/StorageItem Object Reference") (StackIn :type "/Game/Blueprints/Storage/Items/StorageItem Object Reference"))
  (locals (L_Item :type "/Game/Blueprints/Storage/Items/StorageItem Object Reference") (L_StackIn :type "/Game/Blueprints/Storage/Items/StorageItem Object Reference"))
  ;[1 1 1] Stack item
  (set `local.L_Item` Item)
  (bind _output_get (set `local.L_StackIn` StackIn))
  (bind _changed (`/Game/Blueprints/Storage/Items/StorageItem.ChangeCount` _output_get (`/Game/Blueprints/Storage/Items/StorageItem.Count` (`local.L_Item`))))
  (if _changed
    (`self.ChangeTotalWeight` (`/Game/Blueprints/Storage/Items/StorageItem.GetItemWeight` (`local.L_Item`) true 0))))